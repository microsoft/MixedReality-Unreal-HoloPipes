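; BP_PipeGrid is the root actor of the pipes puzzle grid, handling its placement, cursor display and Toolbox level and score updates.
; On Tick it snaps to the game mode's computed root transform, then briefly follows it, lerping small moves and snapping large ones, until a timer locks placement.
; It spawns manipulation, target and connection cursors for left and right, routing cursor state updates to each set.
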(event `self.ReceiveBeginPlay`
  (`self.InitCursors`))

(event `self.OnCursorUpdated`
  (params (state :type "CursorState Structure"))
  (`self.HandleCursorUpdate` state))

(event `self.ReceiveTick`
  (params (DeltaSeconds :type "Float (single-precision)"))
  (bind _location (.location (`SceneComponent.K2_GetComponentToWorld` (`self.DefaultSceneRoot`))))
  (if (`self.PlacementStarted`)
    (if (not (`self.Placed`))
      (bind _asbp_pipes_game_mode (cast `/Game/Blueprints/BP_PipesGameMode` (`GameplayStatics.GetGameMode`)))
      (bind (_transformvalid _transform) (`/Game/Blueprints/BP_PipesGameMode.ComputePipeRootTransform` _asbp_pipes_game_mode))
      (if _transformvalid
        (bind _location_2 (.location _transform))
        (bind _rotation (.rotation _transform))
        (bind _returnvalue (> (`KismetMathLibrary.VSizeSquared` (- _location _location_2)) 10000.0))
        (`SceneComponent.K2_SetWorldTransform` (`self.DefaultSceneRoot`) (`KismetMathLibrary.MakeTransform` (`KismetMathLibrary.SelectVector` _location_2 (`KismetMathLibrary.VLerp` _location _location_2 0.05) _returnvalue) (`KismetMathLibrary.SelectRotator` _rotation (`KismetMathLibrary.RLerp` (.rotation (`SceneComponent.K2_GetComponentToWorld` (`self.DefaultSceneRoot`))) _rotation 0.05 true) _returnvalue) (.scale _transform)) false false)))
    (else
      (bind _asbp_pipes_game_mode_2 (cast `/Game/Blueprints/BP_PipesGameMode` (`GameplayStatics.GetGameMode`)))
      (bind _pawn (`/Game/Blueprints/BP_PipesGameMode.GetPawn` _asbp_pipes_game_mode_2))
      (if (`KismetSystemLibrary.IsValid` _pawn)
        (bind (_transformvalid_2 _transform_2) (`/Game/Blueprints/BP_PipesGameMode.ComputePipeRootTransform` _asbp_pipes_game_mode_2))
        (if _transformvalid_2
          (`SceneComponent.K2_SetWorldTransform` (`self.DefaultSceneRoot`) _transform_2 false false)
          (set `self.PlacementStarted` true)
          (`KismetSystemLibrary.K2_SetTimerDelegate` (delegate `SetPlaced`) 0.25))))))

(event `SetPlaced`
  (set `self.Placed` true))

(fn `HandleConnectionsCursorUpdate`
  (params (State :type "ConnectionsCursorState Structure") (RotateState :type "RotateCursorState Structure") (Cursor :type "/Game/Blueprints/Cursor/BP_ConnectionsCursor Object Reference"))
  (bind (_phase _location _directions _dirty) (break `ConnectionsCursorState` State))
  (if _dirty
    (`/Game/Blueprints/Cursor/BP_ConnectionsCursor.SetCursorState` Cursor _directions _phase (`.Phase` (break `RotateCursorState` RotateState)))
    (if (!= _directions 0)
      (`SceneComponent.K2_SetRelativeLocation` (`/Game/Blueprints/Cursor/BP_ConnectionsCursor.DefaultSceneRoot` Cursor) _location false false))))

(fn `HandleCursorUpdate`
  (params (State :type "CursorState Structure"))
  (bind (_left _right) (break `CursorState` State))
  (bind (_target _translate _rotate _connections) (break `CursorStateHand` _right))
  (bind (_target_2 _translate_2 _rotate_2 _connections_2) (break `CursorStateHand` _left))
  (`|ExecutionSequence`
    (:`then_0`
      (`/Game/Blueprints/Cursor/BP_TargetCursor.UpdateState` (`self.TargetCursor0`) _target_2)
      (`/Game/Blueprints/Cursor/BP_ManipulationCursor.UpdateCursor` (`self.ManipCursor0`) _left)
      (`self.HandleConnectionsCursorUpdate` _connections_2 _rotate_2 (`self.ConnectionCursor0`)))
    (:`then_1`
      (`/Game/Blueprints/Cursor/BP_TargetCursor.UpdateState` (`self.TargetCursor1`) _target)
      (`/Game/Blueprints/Cursor/BP_ManipulationCursor.UpdateCursor` (`self.ManipCursor1`) _right)
      (`self.HandleConnectionsCursorUpdate` _connections _rotate (`self.ConnectionCursor1`)))))

(fn `HandleTargetCursorUpdate`
  (params (State :type "SimpleCursorState Structure") (Mesh :type "StaticMeshComponent Object Reference") (Material :type "MaterialInstanceDynamic Object Reference"))
  (locals (CursorTargetColor :type "LinearColor Structure"))
  (bind (_phase _location _dirty) (break `SimpleCursorState` State))
  (if _dirty
    (switch `EInteractionPhase` _phase
      (:`None`
        (`SceneComponent.SetVisibility` Mesh false false))
      (:`Visible`
        (set `local.CursorTargetColor` (struct :`R` 0.1 :`G` 0.1 :`B` 0.1 :`A` 1.0) :!label _label)
        (`SceneComponent.SetVisibility` Mesh true false :!label _label_2)
        (`SceneComponent.K2_SetRelativeLocation` Mesh _location false false)
        (`MaterialInstanceDynamic.SetVectorParameterValue` Material "Color" (`local.CursorTargetColor`)))
      (:`Pending`
        (goto _label))
      (:`Blocked`
        (goto _label))
      (:`Ready`
        (set `local.CursorTargetColor` (struct :`R` 0.5 :`G` 0.5 :`A` 1.0))
        (goto _label_2)))))

(fn `InitCursors`
  (locals (DefaultTransform :type "Transform Structure"))
  (bind _defaulttransform (`local.DefaultTransform`))
  (bind _defaulttransform_2 (`local.DefaultTransform`))
  (`|ExecutionSequence`
    (:`then_0`
      (bind _returnvalue (`|SpawnActorFromClass` "/Game/Blueprints/Cursor/BP_ManipulationCursor.BP_ManipulationCursor_C" (`local.DefaultTransform`) "AlwaysSpawn" "OverrideRootScale" null null))
      (bind _output_get (set `self.ManipCursor0` _returnvalue))
      (`self.K2_AttachToActor` _output_get self "None" "KeepRelative" "KeepRelative" "KeepRelative" false)
      (bind _returnvalue_2 (`|SpawnActorFromClass` "/Game/Blueprints/Cursor/BP_ManipulationCursor.BP_ManipulationCursor_C" (`local.DefaultTransform`) "AlwaysSpawn" "OverrideRootScale" null null))
      (bind _output_get_2 (set `self.ManipCursor1` _returnvalue_2))
      (`self.K2_AttachToActor` _output_get_2 self "None" "KeepRelative" "KeepRelative" "KeepRelative" false))
    (:`then_1`
      (bind _returnvalue_3 (`|SpawnActorFromClass` "/Game/Blueprints/Cursor/BP_TargetCursor.BP_TargetCursor_C" _defaulttransform_2 "AlwaysSpawn" "OverrideRootScale" null null))
      (set `self.TargetCursor0` _returnvalue_3)
      (bind _returnvalue_4 (`|SpawnActorFromClass` "/Game/Blueprints/Cursor/BP_TargetCursor.BP_TargetCursor_C" _defaulttransform_2 "AlwaysSpawn" "OverrideRootScale" null null))
      (set `self.TargetCursor1` _returnvalue_4))
    (:`then_2`
      (bind _returnvalue_5 (`|SpawnActorFromClass` "/Game/Blueprints/Cursor/BP_ConnectionsCursor.BP_ConnectionsCursor_C" _defaulttransform "AlwaysSpawn" "OverrideRootScale" null null))
      (bind _output_get_3 (set `self.ConnectionCursor0` _returnvalue_5))
      (`self.K2_AttachToActor` _output_get_3 self "None" "KeepRelative" "KeepRelative" "KeepRelative" false)
      (bind _returnvalue_6 (`|SpawnActorFromClass` "/Game/Blueprints/Cursor/BP_ConnectionsCursor.BP_ConnectionsCursor_C" _defaulttransform "AlwaysSpawn" "OverrideRootScale" null null))
      (bind _output_get_4 (set `self.ConnectionCursor1` _returnvalue_6))
      (`self.K2_AttachToActor` _output_get_4 self "None" "KeepRelative" "KeepRelative" "KeepRelative" false))))

(fn `SetLevel`
  (params (Number :type Integer) (Enable :type Boolean))
  (bind _toolbox (`self.Toolbox`))
  (if (`KismetSystemLibrary.IsValid` _toolbox)
    (bind _asbp_toolbox (cast `/Game/Blueprints/Toolbox/BP_Toolbox` _toolbox))
    (`/Game/Blueprints/Toolbox/BP_Toolbox.SetLevel` _asbp_toolbox Number))
  (`self.SetInteractionEnabled` Enable))

(fn `SetScore`
  (params (Number :type Integer))
  (bind _toolbox (`self.Toolbox`))
  (if (`KismetSystemLibrary.IsValid` _toolbox)
    (bind _asbp_toolbox (cast `/Game/Blueprints/Toolbox/BP_Toolbox` _toolbox))
    (`/Game/Blueprints/Toolbox/BP_Toolbox.SetScore` _asbp_toolbox Number)))

(fn `ShowWorldCursor`
  (params (Size :type Integer) (Visible :type Boolean))
  (bind _worldcursor (`self.WorldCursor`))
  (bind _returnvalue (select `bool` (== (mod Size 2) 0) :`true` (* (`self.CellSize`) -0.5)))
  (`SceneComponent.SetRelativeScale3D` _worldcursor (* (0.4 0.4 0.4) Size))
  (`SceneComponent.K2_SetRelativeLocation` _worldcursor (`KismetMathLibrary.MakeVector` _returnvalue _returnvalue _returnvalue) false false)
  (`SceneComponent.SetVisibility` _worldcursor Visible false))

(fn `UserConstructionScript`)