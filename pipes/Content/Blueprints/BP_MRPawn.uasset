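; Mixed-reality player pawn for HoloPipes that turns hand tracking, eye gaze and voice commands into interaction.
; Each tick it derives pinch and gaze state, falling back to camera gaze and warning when eye tracking is lost.
; Two BP_Fingertip actors compete for registered interactables, with duplicate-target arbitration and optional focus capture.
; Voice input actions are broadcast as keyword events, spawning a tooltip when handled.
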(event `self.ReceiveBeginPlay`
  (bind _returnvalue (`KismetMathLibrary.MakeTransform` (0.0 0.0 0.0)))
  (bind _fingertips (`self.Fingertips`))
  (`|ExecutionSequence`
    (:`then_0`
      (set `self.VRCamera` (`self.Camera`)))
    (:`then_1`
      (bind _returnvalue_2 (`|SpawnActorFromClass` "/Game/Blueprints/Buttons/BP_Fingertip.BP_Fingertip_C" _returnvalue "Undefined" "OverrideRootScale" null "Left" "IndexTip" "IndexDistal" null))
      (`KismetArrayLibrary.Array_Add` _fingertips _returnvalue_2))
    (:`then_2`
      (bind _returnvalue_3 (`|SpawnActorFromClass` "/Game/Blueprints/Buttons/BP_Fingertip.BP_Fingertip_C" _returnvalue "Undefined" "OverrideRootScale" null "Right" "IndexTip" "IndexDistal" null))
      (`KismetArrayLibrary.Array_Add` _fingertips _returnvalue_3))))

(event `self.ReceiveTick`
  (params (DeltaSeconds :type "Float (single-precision)"))
  (bind (_origin _direction) (`self.DetectGazeState`))
  (bind (_pose _target _attach) (`self.DetectHandState` "Right"))
  (bind (_pose_2 _target_2 _attach_2) (`self.DetectHandState` "Left"))
  (set `self.CurrentlyGrasped` (or (`|EnumEquality` _pose "Pinched") (`|EnumEquality` _pose_2 "Pinched")))
  (`self.UpdateFingerState` (make `FingersUpdate` (make `FingerUpdate` _pose_2 _target_2 _attach_2) (make `FingerUpdate` _pose _target _attach)) (make `GazeUpdate` _origin _direction))
  (`self.UpdateFocus`))

(event `InputAction|LeftGrasp`
  (params (Key :type "Key Structure"))
  (:`Pressed`
    (set `self.LeftGraspReported` true))
  (:`Released`
    (set `self.LeftGraspReported` false)))

(event `InputAction|RightGrasp`
  (params (Key :type "Key Structure"))
  (:`Pressed`
    (set `self.RightGraspReported` true))
  (:`Released`
    (set `self.RightGraspReported` false)))

(event `/Game/Blueprints/Buttons/Interface_EventSource.EventHandled`
  (set `self.CurrentEventHandled` true))

(event `InputAction|Yes`
  (params (Key :type "Key Structure"))
  (:`Pressed`
    (`self.FireVoiceEvent` "NewEnumerator0")))

(event `InputAction|No`
  (params (Key :type "Key Structure"))
  (:`Pressed`
    (`self.FireVoiceEvent` "NewEnumerator1")))

(event `InputAction|GotIt`
  (params (Key :type "Key Structure"))
  (:`Pressed`
    (`self.FireVoiceEvent` "NewEnumerator2")))

(event `InputAction|Next`
  (params (Key :type "Key Structure"))
  (:`Pressed`
    (`self.FireVoiceEvent` "NewEnumerator3")))

(event `InputAction|Previous`
  (params (Key :type "Key Structure"))
  (:`Pressed`
    (`self.FireVoiceEvent` "NewEnumerator10")))

(event `InputAction|ShowCursor`
  (params (Key :type "Key Structure"))
  (:`Pressed`
    (`self.FireVoiceEvent` "NewEnumerator4")))

(event `InputAction|HideCursor`
  (params (Key :type "Key Structure"))
  (:`Pressed`
    (`self.FireVoiceEvent` "NewEnumerator11")))

(event `InputAction|ShowLabels`
  (params (Key :type "Key Structure"))
  (:`Pressed`
    (`self.FireVoiceEvent` "NewEnumerator9")))

(event `InputAction|HideLabels`
  (params (Key :type "Key Structure"))
  (:`Pressed`
    (`self.FireVoiceEvent` "NewEnumerator12")))

(event `InputAction|MoveGame`
  (params (Key :type "Key Structure"))
  (:`Pressed`
    (`self.FireVoiceEvent` "NewEnumerator5")))

(event `InputAction|PlaceGame`
  (params (Key :type "Key Structure"))
  (:`Pressed`
    (`self.FireVoiceEvent` "NewEnumerator13")))

(event `InputAction|RecallGame`
  (params (Key :type "Key Structure"))
  (:`Pressed`
    (`self.FireVoiceEvent` "NewEnumerator6")))

(event `InputAction|SweepLevel`
  (params (Key :type "Key Structure"))
  (:`Pressed`
    (`self.FireVoiceEvent` "NewEnumerator7")))

(event `InputAction|ImportGame`
  (params (Key :type "Key Structure"))
  (:`Pressed`
    (`self.FireVoiceEvent` "NewEnumerator15")))

(event `InputAction|ExportGame`
  (params (Key :type "Key Structure"))
  (:`Pressed`
    (`self.FireVoiceEvent` "NewEnumerator14")))

(event `InputAction|DebugToggleFocus`
  (params (Key :type "Key Structure"))
  (:`Pressed`
    (`self.FireVoiceEvent` "NewEnumerator16")))

(event `InputAction|ScrollUp`
  (params (Key :type "Key Structure"))
  (:`Pressed`
    (`self.FireVoiceEvent` "NewEnumerator18")))

(event `InputAction|ScrollDown`
  (params (Key :type "Key Structure"))
  (:`Pressed`
    (`self.FireVoiceEvent` "NewEnumerator19")))

(event `InputAction|SkipLevel`
  (params (Key :type "Key Structure"))
  (:`Pressed`
    (`self.FireVoiceEvent` "NewEnumerator20")))

(event `InputAction|MainMenu`
  (params (Key :type "Key Structure"))
  (:`Pressed`
    (`self.FireVoiceEvent` "NewEnumerator17")))

(fn `AddInteractable`
  (params (Interactable :type "/Game/Blueprints/Buttons/Interface_Interactable Interface"))
  (bind _returnvalue (`KismetSystemLibrary.Conv_InterfaceToObject` Interactable))
  (bind _has (`self.HasInteractable` Interactable))
  (if _has
    _
    (elif (`KismetSystemLibrary.IsValid` _returnvalue)
      (`BlueprintSetLibrary.Set_Add` (`self.TargetsSet`) _returnvalue)
      (`self.RebuildTargets`))))

(fn `AnyInteractableFocused`
  (returns (Focused :type Boolean))
  (bind _fingertips (`self.Fingertips`))
  (return (or (`.Valid_20_591A6B194CD54A976F20ACBAAE539A21` (break `/Game/Blueprints/Buttons/STRUCT_FocusTarget` (`/Game/Blueprints/Buttons/BP_Fingertip.CurrentTarget` (`|GetArrayItem` _fingertips)))) (`.Valid_20_591A6B194CD54A976F20ACBAAE539A21` (break `/Game/Blueprints/Buttons/STRUCT_FocusTarget` (`/Game/Blueprints/Buttons/BP_Fingertip.CurrentTarget` (`|GetArrayItem` _fingertips 1)))))))

(fn `CaptureFocus`
  (params (Captured :type "/Game/Blueprints/Buttons/Interface_Interactable Interface") (Hand :type "EControllerHand Enum" :default "Left"))
  (locals (Fingertip :type "/Game/Blueprints/Buttons/BP_Fingertip Object Reference") (Index :type Integer) (HasCaptured :type Boolean) (DistSqToCaptured :type "Float (double-precision)"))
  (bind (_currenttarget_valid _currenttarget_target _currenttarget_type _currenttarget_cursor _currenttarget_point _currenttarget_normal _currenttarget_distancesq) (break `/Game/Blueprints/Buttons/STRUCT_FocusTarget` (`/Game/Blueprints/Buttons/BP_Fingertip.CurrentTarget` (`local.Fingertip`))))
  (bind (_valid _target) (break `/Game/Blueprints/Buttons/STRUCT_FocusTarget` (`/Game/Blueprints/Buttons/BP_Fingertip.CurrentTarget` (`local.Fingertip`))))
  (bind _has (`self.HasInteractable` Captured))
  (if _has
    (if (`self.FocusCaptured`)
      (`/Game/Blueprints/Buttons/Interface_Interactable.UpdateFocusPoint` (`self.FocusCapturedTarget`) "NewEnumerator2" (0.0 0.0 0.0)))
    (set `self.FocusCaptured` true)
    (set `self.FocusCapturedTarget` (`local.Captured`))
    (set `self.FocusCapturedIndexValid` false)
    (for (_array_element _array_index) (`self.Fingertips`)
      (set `local.Fingertip` _array_element)
      (set `local.Index` _array_index)
      (bind _equal (`self.InteractablesEqual` (`local.Captured`) _target))
      (set `local.HasCaptured` (and _equal _valid))
      (switch `EControllerHand` (`local.Hand`)
        (:`Left`
          (if (`|EnumEquality` (`local.Hand`) (`/Game/Blueprints/Buttons/BP_Fingertip.Hand` (`local.Fingertip`))) :!label _label
            (set `self.FocusCapturedIndex` (`local.Index`))
            (set `self.FocusCapturedIndexValid` true)
            (if (not (`local.HasCaptured`))
              (`/Game/Blueprints/Buttons/BP_Fingertip.ClearFocus` (`local.Fingertip`) (not (`local.HasCaptured`)) :!label _label_2))
            (else
              (goto _label_2))))
        (:`Right`
          (goto _label))
        (:`AnyHand`
          (if (not (`local.HasCaptured`))
            (goto _label_2)
            (else
              (if (`self.FocusCapturedIndexValid`)
                (if (> (`local.DistSqToCaptured`) _currenttarget_distancesq)
                  (`/Game/Blueprints/Buttons/BP_Fingertip.ClearFocus` (`|GetArrayItem` (`self.Fingertips`) (`self.FocusCapturedIndex`)) false)
                  (else
                    (goto _label_2))))
              (set `self.FocusCapturedIndex` (`local.Index`))
              (set `self.FocusCapturedIndexValid` true)
              (set `local.DistSqToCaptured` _currenttarget_distancesq))))))))

(fn `DetectGazeState`
  (returns (Origin :type "Vector Structure") (Direction :type "Vector Structure"))
  (bind _camera (`self.Camera`))
  (bind (_outgazedata _returnvalue) (`EyeTrackerFunctionLibrary.GetGazeData`))
  (`self.Handle Have Eye Gaze` _returnvalue)
  (bind (_gazeorigin _gazedirection) (break `EyeTrackerGazeData` _outgazedata))
  (return (`KismetMathLibrary.SelectVector` _gazeorigin (`SceneComponent.K2_GetComponentLocation` _camera) _returnvalue) (`KismetMathLibrary.SelectVector` _gazedirection (`SceneComponent.GetForwardVector` _camera) _returnvalue)))

(fn `DetectHandState`
  (params (Hand :type "EControllerHand Enum" :default "Left"))
  (returns (Pose :type "EFingerPose Enum") (Target :type "Transform Structure") (Attach :type "Transform Structure"))
  (locals (FingerPose :type "EFingerPose Enum") (TargetTransform :type "Transform Structure") (AttachTransform :type "Transform Structure") (TransformsFresh :type Boolean))
  (bind _returnvalue (`KismetMathLibrary.Conv_ByteToInt` (enumliteral `EHandKeypoint` "ThumbProximal")))
  (bind _returnvalue_2 (`KismetMathLibrary.Conv_ByteToInt` (enumliteral `EHandKeypoint` "ThumbTip")))
  (bind _returnvalue_3 (`KismetMathLibrary.Conv_ByteToInt` (enumliteral `EHandKeypoint` "LittleTip")))
  (bind _returnvalue_4 (`KismetMathLibrary.Conv_ByteToInt` (enumliteral `EHandKeypoint` "Palm")))
  (`|ExecutionSequence`
    (:`then_0`
      (bind _motioncontrollerdata (`HeadMountedDisplayFunctionLibrary.GetMotionControllerData` null Hand))
      (bind (_bvalid _devicename _applicationinstanceid _devicevisualtype _handindex _trackingstatus _gripposition _griprotation _aimposition _aimrotation _handkeypositions _handkeyrotations) (break `XRMotionControllerData` _motioncontrollerdata))
      (bind _output_get (set `local.TransformsFresh` (and _bvalid (`|EnumEquality` _devicevisualtype "Hand"))))
      (if _output_get
        (bind _output (`|GetArrayItem` _handkeypositions _returnvalue_3))
        (bind _returnvalue_5 (`KismetMathLibrary.MakeTransform` _output (`KismetMathLibrary.Quat_Rotator` (`|GetArrayItem` _handkeyrotations _returnvalue_3))))
        (bind _output_2 (`|GetArrayItem` _handkeypositions _returnvalue_2))
        (bind _output_3 (`|GetArrayItem` _handkeypositions _returnvalue))
        (set `local.TargetTransform` (select `bool` (> (`KismetMathLibrary.VSizeSquared` (- _output_2 _output)) (`KismetMathLibrary.VSizeSquared` (- _output _output_3))) :`false` (`KismetMathLibrary.TLerp` _returnvalue_5 (`KismetMathLibrary.MakeTransform` _output_2 (`KismetMathLibrary.Quat_Rotator` (`|GetArrayItem` _handkeyrotations _returnvalue_2))) 0.5) :`true` (`KismetMathLibrary.TLerp` _returnvalue_5 (`KismetMathLibrary.MakeTransform` _output_3 (`KismetMathLibrary.Quat_Rotator` (`|GetArrayItem` _handkeyrotations _returnvalue))) 0.5)))
        (set `local.AttachTransform` (`KismetMathLibrary.MakeTransform` (`|GetArrayItem` _handkeypositions _returnvalue_4) (`KismetMathLibrary.Quat_Rotator` (`|GetArrayItem` _handkeyrotations _returnvalue_4))))))
    (:`then_1`
      (if (`local.TransformsFresh`)
        (set `local.FingerPose` (select `bool` (select `bool` (`|EnumEquality` Hand "Left") :`false` (`self.RightGraspReported`) :`true` (`self.LeftGraspReported`)) :`false` "Tracked" :`true` "Pinched" :!type "EFingerPose Enum"))))
    (:`then_2`
      (return (`local.FingerPose`) (`local.TargetTransform`) (`local.AttachTransform`)))))

(fn `FireVoiceEvent`
  (params (Keyword :type "/Game/Blueprints/Buttons/ENUM_VoiceInput Enum" :default "NewEnumerator0"))
  (set `self.CurrentEventHandled` false)
  (`self.VoiceInputDispatcher` Keyword self)
  (if (`self.CurrentEventHandled`)
    (bind _text (`self.VoiceKeywordToText` Keyword))
    (`|SpawnActorFromClass` "/Game/Blueprints/Buttons/BP_VoiceTooltip.BP_VoiceTooltip_C" (`KismetMathLibrary.MakeTransform` (0.0 0.0 0.0)) "AlwaysSpawn" "OverrideRootScale" null _text null)))

(fn `GenerateNewLevel`
  (params (LevelModifier :type Integer) (ToggleSolution :type Boolean))
  (bind _asppipes_game_mode (cast `PPipesGameMode` (`GameplayStatics.GetGameMode`)))
  (`PPipesGameMode.GenerateLevel` _asppipes_game_mode (+ (`PPipesGameMode.Level` _asppipes_game_mode) LevelModifier) (!= (`PPipesGameMode.GenerateLevelSolution` _asppipes_game_mode) ToggleSolution)))

(fn `Handle Have Eye Gaze`
  (params (Gaze :type Boolean))
  (if Gaze
    (set `self.LastSawGaze` (`GameplayStatics.GetTimeSeconds`))
    (if (not (`self.CurrentlyHaveGaze`))
      (if (`KismetSystemLibrary.IsValid` (`self.EyeTrackingLostDialog`))
        (if (>= (- (`GameplayStatics.GetTimeSeconds`) (`self.GazeDialogShown`)) (`self.MinGazeDialogTime`))
          (set `self.CurrentlyHaveGaze` true)
          (`self.K2_DestroyActor` (`self.EyeTrackingLostDialog`)))
        (else
          (set `self.CurrentlyHaveGaze` true))))
    (elif (and (>= (- (`GameplayStatics.GetTimeSeconds`) (`self.LastSawGaze`)) (`self.GazeLostTime`)) (`self.CurrentlyHaveGaze`))
      (set `self.CurrentlyHaveGaze` false)
      (bind _returnvalue (`|SpawnActorFromClass` "/Game/Blueprints/Dialogs/BP_Dialog_Error.BP_Dialog_Error_C" (`KismetMathLibrary.MakeTransform` (0.0 0.0 0.0)) "Undefined" "OverrideRootScale" null null))
      (bind _output_get (set `self.EyeTrackingLostDialog` _returnvalue))
      (set `/Game/Blueprints/Dialogs/BP_Dialog.ShowPlaysSound` false _output_get)
      (`/Game/Blueprints/Dialogs/BP_Dialog_Error.ShowErrorDialog` _output_get "We can't see your eyes! \n \nHoloPipes requires eye tracking for the best experience. If you see this message frequently, please calibrate eye tracking in System Settings.")
      (set `self.GazeDialogShown` (`GameplayStatics.GetTimeSeconds`)))))

(fn `HasInteractable`
  (params (Interactable :type "/Game/Blueprints/Buttons/Interface_Interactable Interface"))
  (returns (Has :type Boolean))
  (return (`BlueprintSetLibrary.Set_Contains` (`self.TargetsSet`) (`KismetSystemLibrary.Conv_InterfaceToObject` Interactable))))

(fn `InteractablesEqual`
  (params (A :type "/Game/Blueprints/Buttons/Interface_Interactable Interface") (B :type "/Game/Blueprints/Buttons/Interface_Interactable Interface"))
  (returns (Equal :type Boolean))
  (return (== (`KismetSystemLibrary.Conv_InterfaceToObject` A) (`KismetSystemLibrary.Conv_InterfaceToObject` B))))

(fn `IsCurrentlyGrasped`
  (returns (Grasped :type Boolean))
  (return (`self.CurrentlyGrasped`)))

(fn `RebuildTargets`
  (`KismetArrayLibrary.Array_Clear` (`self.Targets`))
  (bind _result (`BlueprintSetLibrary.Set_ToArray` (`self.TargetsSet`)))
  (for _array_element _result
    (bind _asinterface_interactable (cast `/Game/Blueprints/Buttons/Interface_Interactable` _array_element))
    (`KismetArrayLibrary.Array_Add` (`self.Targets`) _asinterface_interactable)))

(fn `ReleaseFocus`
  (params (Released :type "/Game/Blueprints/Buttons/Interface_Interactable Interface"))
  (if (`self.FocusCaptured`)
    (bind _equal (`self.InteractablesEqual` (`local.Released`) (`self.FocusCapturedTarget`)))
    (if _equal
      (set `self.FocusCaptured` false)
      (set `self.FocusCapturedIndexValid` false)
      (set `self.FocusCapturedTarget` null)
      (for _array_element (`self.Fingertips`)
        (bind _equal_2 (`self.InteractablesEqual` (`local.Released`) (`.Target_7_9D770DD34598AAE6CF527E8DAE188FDC` (break `/Game/Blueprints/Buttons/STRUCT_FocusTarget` (`/Game/Blueprints/Buttons/BP_Fingertip.CurrentTarget` _array_element)))))
        (if _equal_2
          (`/Game/Blueprints/Buttons/BP_Fingertip.ClearFocus` _array_element true))))))

(fn `RemoveInteractable`
  (params (Interactable :type "/Game/Blueprints/Buttons/Interface_Interactable Interface"))
  (`self.HasInteractable` Interactable)
  (if true
    (`BlueprintSetLibrary.Set_Remove` (`self.TargetsSet`) (`KismetSystemLibrary.Conv_InterfaceToObject` Interactable))
    (`self.RebuildTargets`)
    (`self.ReleaseFocus` (`local.Interactable`))))

(fn `UpdateFocus`
  (locals (CurrentFingertip :type "/Game/Blueprints/Buttons/BP_Fingertip Object Reference") (Fingertip0 :type "/Game/Blueprints/Buttons/BP_Fingertip Object Reference") (Fingertip1 :type "/Game/Blueprints/Buttons/BP_Fingertip Object Reference") (Announce0 :type Boolean) (Announce1 :type Boolean) (ShouldAnnounceClear :type Boolean))
  (bind _focuscapturedindexvalid (`self.FocusCapturedIndexValid`))
  (bind _fingertips (`self.Fingertips`))
  (`|ExecutionSequence`
    (:`then_0`
      (for (_array_element _array_index) (`self.Fingertips`)
        (bind _output_get (set `local.CurrentFingertip` _array_element))
        (if (`/Game/Blueprints/Buttons/BP_Fingertip.PointerLocationValid` _output_get)
          (if (not (`self.FocusCaptured`))
            (for _array_element_2 (`self.Targets`)
              (`/Game/Blueprints/Buttons/BP_Fingertip.ConsiderForFocus` (`local.CurrentFingertip`) _array_element_2))
            (elif (or (and (== _array_index (`self.FocusCapturedIndex`)) _focuscapturedindexvalid) (not _focuscapturedindexvalid))
              (`/Game/Blueprints/Buttons/BP_Fingertip.ConsiderForFocus` (`local.CurrentFingertip`) (`self.FocusCapturedTarget`)))))))
    (:`then_1`
      (for _array_element_3 (`self.Fingertips`)
        (bind _output_get_2 (set `local.CurrentFingertip` _array_element_3))
        (bind _currenttarget_valid (break `/Game/Blueprints/Buttons/STRUCT_FocusTarget` (`/Game/Blueprints/Buttons/BP_Fingertip.CurrentTarget` _output_get_2)))
        (if _currenttarget_valid
          (set `local.ShouldAnnounceClear` true)
          (for _array_element_4 (`self.Fingertips`)
            (bind (_valid _target) (break `/Game/Blueprints/Buttons/STRUCT_FocusTarget` (`/Game/Blueprints/Buttons/BP_Fingertip.NextTarget` _array_element_4)))
            (if _valid
              (bind _equal (`self.InteractablesEqual` _target (`.Target_7_9D770DD34598AAE6CF527E8DAE188FDC` (break `/Game/Blueprints/Buttons/STRUCT_FocusTarget` (`/Game/Blueprints/Buttons/BP_Fingertip.CurrentTarget` (`local.CurrentFingertip`))))))
              (if _equal
                (set `local.ShouldAnnounceClear` false))))
          (`/Game/Blueprints/Buttons/BP_Fingertip.Clear Stale Focus` (`local.CurrentFingertip`) (`local.ShouldAnnounceClear`)))))
    (:`then_2`
      (`|ExecutionSequence`
        (:`then_0`
          (bind _output_get_3 (set `local.Fingertip0` (`|GetArrayItem` _fingertips)))
          (set `local.Announce0` (`.Valid_20_591A6B194CD54A976F20ACBAAE539A21` (break `/Game/Blueprints/Buttons/STRUCT_FocusTarget` (`/Game/Blueprints/Buttons/BP_Fingertip.NextTarget` _output_get_3))))
          (bind _output_get_4 (set `local.Fingertip1` (`|GetArrayItem` _fingertips 1)))
          (set `local.Announce1` (`.Valid_20_591A6B194CD54A976F20ACBAAE539A21` (break `/Game/Blueprints/Buttons/STRUCT_FocusTarget` (`/Game/Blueprints/Buttons/BP_Fingertip.NextTarget` _output_get_4)))))
        (:`then_1`
          (if (and (`local.Announce0`) (`local.Announce1`))
            (bind _equal_2 (`self.InteractablesEqual` (`.Target_7_9D770DD34598AAE6CF527E8DAE188FDC` (break `/Game/Blueprints/Buttons/STRUCT_FocusTarget` (`/Game/Blueprints/Buttons/BP_Fingertip.NextTarget` (`local.Fingertip0`)))) (`.Target_7_9D770DD34598AAE6CF527E8DAE188FDC` (break `/Game/Blueprints/Buttons/STRUCT_FocusTarget` (`/Game/Blueprints/Buttons/BP_Fingertip.NextTarget` (`local.Fingertip1`))))))
            (if _equal_2
              (bind _choose (`/Game/Blueprints/Buttons/BP_Fingertip.Choose Candidate Over Next` (`local.Fingertip0`) (`/Game/Blueprints/Buttons/BP_Fingertip.NextTarget` (`local.Fingertip1`)) false))
              (bind _output_get_5 (set `local.Announce1` _choose))
              (set `local.Announce0` (not _output_get_5)))))
        (:`then_2`
          (if (and (`self.FocusCaptured`) (not (`self.FocusCapturedIndexValid`)))
            (bind _output_get_6 (set `self.FocusCapturedIndexValid` (or (`local.Announce0`) (`local.Announce1`))))
            (if _output_get_6
              (if (`local.Announce0`)
                (set `self.FocusCapturedIndex` 0)
                (`/Game/Blueprints/Buttons/BP_Fingertip.ClearFocus` (`local.Fingertip1`) false)
                (else
                  (set `self.FocusCapturedIndex` 1)
                  (`/Game/Blueprints/Buttons/BP_Fingertip.ClearFocus` (`local.Fingertip0`) false))))))
        (:`then_3`
          (`/Game/Blueprints/Buttons/BP_Fingertip.CommitNewFocus` (`local.Fingertip0`) (`local.Announce0`))
          (`/Game/Blueprints/Buttons/BP_Fingertip.CommitNewFocus` (`local.Fingertip1`) (`local.Announce1`)))))))

(fn `UserConstructionScript`)

(fn `VoiceKeywordToText`
  (params (Keyword :type "/Game/Blueprints/Buttons/ENUM_VoiceInput Enum" :default "NewEnumerator0"))
  (returns (Text :type Text))
  (return (`KismetTextLibrary.Conv_StringToText` (`|GetEnumeratorNameAsString` Keyword))))