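; BP_DynamicText renders configurable text into a canvas render target texture at runtime.
; Setters store text, size, colors, font size and alignment, then request a redraw, optional for all but text.
; The update request recreates the render target only when it is invalid or its dimensions change, binds its update event, then refreshes it.
; The canvas update fills the background and draws vertically centered text, aligned horizontally, in a normal or large font.
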(fn `Request Canvas Update`
  (bind (_width _height) (`CanvasRenderTarget2D.GetSize` (`self.Texture`)))
  (if (`KismetSystemLibrary.IsValid` (`self.Texture`))
    (if (not (and (== (`self.TextureWidth`) _width) (== _height (`self.TextureHeight`))))
      (bind _returnvalue (`CanvasRenderTarget2D.CreateCanvasRenderTarget2D` "/Script/Engine.CanvasRenderTarget2D" (`self.TextureWidth`) (`self.TextureHeight`) :!label _label))
      (bind _output_get (set `self.Texture` _returnvalue))
      (add `CanvasRenderTarget2D.OnCanvasRenderTargetUpdate` _output_get (`|CreateDelegate` :!event `UpdateCanvas`)))
    (else
      (goto _label)))
  (`CanvasRenderTarget2D.UpdateResource` (`self.Texture`)))

(fn `SetTextAlignment`
  (params (Align :type "EHorizontalAlignment Enum" :default "HAlign_Fill") (Redraw :type Boolean))
  (set `self.Alignment` Align)
  (if Redraw
    (`self.Request Canvas Update`)))

(fn `SetTextSize`
  (params (Large :type Boolean) (Redraw :type Boolean))
  (set `self.TextLarge` Large)
  (if Redraw
    (`self.Request Canvas Update`)))

(fn `SetTextureBackColor`
  (params (Color :type "LinearColor Structure") (Redraw :type Boolean))
  (set `self.BackColor` Color)
  (if Redraw
    (`self.Request Canvas Update`)))

(fn `SetTextureForeColor`
  (params (Color :type "LinearColor Structure") (Redraw :type Boolean))
  (set `self.ForeColor` Color)
  (if Redraw
    (`self.Request Canvas Update`)))

(fn `SetTextureSize`
  (params (Width :type Integer) (Height :type Integer) (Redraw :type Boolean))
  (set `self.TextureWidth` Width)
  (set `self.TextureHeight` Height)
  (if Redraw
    (`self.Request Canvas Update`)))

(fn `SetTextureText`
  (params (Text :type Text))
  (set `self.TextureText` Text)
  (`self.Request Canvas Update`))

(fn `UpdateCanvas`
  (params (Canvas :type "Canvas Object Reference") (Width :type Integer) (Height :type Integer))
  (locals (CenterX :type Boolean) (CenterY :type Boolean) (TextX :type "Float (double-precision)") (TextY :type "Float (double-precision)") (Font :type "Font Object Reference"))
  (`Canvas.K2_DrawTexture` Canvas null (0.0 0.0) (`KismetMathLibrary.MakeVector2D` (`KismetMathLibrary.Conv_IntToDouble` Width) (`KismetMathLibrary.Conv_IntToDouble` Height)) (0.0 0.0) (1.0 1.0) (`self.BackColor`) "BLEND_Opaque" 0.0 (0.5 0.5))
  (set `local.Font` (select `bool` (`self.TextLarge`) :`false` "/Game/Blueprints/DynamicText/FONT_DynamicText.FONT_DynamicText" :`true` "/Game/Blueprints/DynamicText/FONT_DynamicTextLarge.FONT_DynamicTextLarge" :!type "Font Object Reference"))
  (set `local.TextY` (/ (`KismetMathLibrary.Conv_IntToDouble` (`local.Height`)) 2.0))
  (set `local.CenterY` true)
  (switch `EHorizontalAlignment` (`self.Alignment`)
    (:`HAlign_Fill`
      (set `local.TextX` (/ (`KismetMathLibrary.Conv_IntToDouble` (`local.Width`)) 2.0) :!label _label)
      (set `local.CenterX` true))
    (:`HAlign_Left`
      (set `local.TextX` 0.0))
    (:`HAlign_Center`
      (goto _label))
    (:`HAlign_Right`
      (bind _returnvalue (`Canvas.K2_TextSize` (`local.Canvas`) (`local.Font`) (`KismetTextLibrary.Conv_TextToString` (`self.TextureText`)) (1.0 1.0)))
      (set `local.TextX` (- (`KismetMathLibrary.Conv_IntToDouble` (`local.Width`)) (`KismetMathLibrary.BreakVector2D` _returnvalue)))))
  (`Canvas.K2_DrawText` (`local.Canvas`) (`local.Font`) (`KismetTextLibrary.Conv_TextToString` (`self.TextureText`)) (`KismetMathLibrary.MakeVector2D` (`local.TextX`) (`local.TextY`)) (1.0 1.0) (`self.ForeColor`) 0.0 (struct :`A` 1.0) (1.0 1.0) (`local.CenterX`) (`local.CenterY`) false (struct)))