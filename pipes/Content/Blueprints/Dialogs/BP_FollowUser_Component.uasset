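; Component that keeps its owning actor, likely a dialog, floating in front of the pawn's camera and facing along the view toward it.
; ComputePosition lazily follows, moving the goal only when it leaves a distance band or view-angle cone, then clamping it back inside.
; UpdatePlacement lerps the owner to that transform, snapping on large jumps or when lerping is disallowed.
; An optional override object can replace the position or lerp decision.
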(fn `CanLerpTransform`
  (returns (CanLerp :type Boolean))
  (if (`self.HasOverride`)
    (bind (_override _canlerp) (`/Game/Blueprints/Dialogs/Interface_FollowUser_Override.CanLerpTransform` (`self.Override`)))
    (if _override
      (return _canlerp)
      (else
        _)))
  (return true))

(fn `Compute Position`
  (params (Initial :type Boolean) (CamPosition :type "Vector Structure") (CamForward :type "Vector Structure"))
  (returns (Location :type "Vector Structure"))
  (locals (CameraPosition :type "Vector Structure") (CameraForward :type "Vector Structure"))
  (bind _returnvalue (`KismetMathLibrary.Vector_DistanceSquared` (`local.CameraPosition`) (`self.LocationGoal`)))
  (bind _returnvalue_2 (`KismetMathLibrary.Normal` (- (`self.LocationGoal`) (`local.CameraPosition`))))
  (bind _returnvalue_3 (`KismetMathLibrary.DegAcos` (`KismetMathLibrary.Dot_VectorVector` (`local.CameraForward`) _returnvalue_2)))
  (bind _returnvalue_4 (>= _returnvalue_3 (`self.MaxDegrees`)))
  (if (`self.HasOverride`)
    (bind (_override _location) (`/Game/Blueprints/Dialogs/Interface_FollowUser_Override.ComputePosition` (`self.Override`) (`local.Initial`) (`local.CamPosition`) (`local.CamForward`)))
    (if _override
      (bind _output_get (set `self.LocationGoal` _location))
      (return _output_get)
      (else
        _)))
  (set `local.CameraPosition` (`local.CamPosition`))
  (set `local.CameraForward` (`local.CamForward`))
  (if (`local.Initial`)
    (bind _output_get_2 (set `self.LocationGoal` (+ (`local.CameraPosition`) (* (`local.CameraForward`) (`self.DesiredDistance`)))))
    (return _output_get_2)
    (else
      (if (not (`KismetMathLibrary.InRange_FloatFloat` _returnvalue (`KismetMathLibrary.Square` (`self.MinDistance`)) (`KismetMathLibrary.Square` (`self.MaxDistance`))))
        _
        (elif _returnvalue_4
          _
          (else
            (return (`self.LocationGoal`)))))
      (bind _output_get_3 (set `self.LocationGoal` (+ (* (`KismetMathLibrary.RotateAngleAxis` _returnvalue_2 (`KismetMathLibrary.SelectFloat` (- _returnvalue_3 (`self.MaxDegrees`)) 0.0 _returnvalue_4) (`KismetMathLibrary.Normal` (`KismetMathLibrary.Cross_VectorVector` _returnvalue_2 (`local.CameraForward`)))) (`KismetMathLibrary.FClamp` (`KismetMathLibrary.Sqrt` _returnvalue) (`self.MinDistance`) (`self.MaxDistance`))) (`local.CameraPosition`))))
      (return _output_get_3))))

(fn `ComputePlacement`
  (params (Initial :type Boolean))
  (returns (TransformValid :type Boolean) (Transform :type "Transform Structure"))
  (locals (CameraPosition :type "Vector Structure") (CameraForward :type "Vector Structure") (CameraValid :type Boolean) (LocationValid :type Boolean) (Location :type "Vector Structure") (Rotation :type "Rotator Structure") (RotationValid :type Boolean))
  (bind _pawn (`self.Pawn`))
  (bind _returnvalue (and (`local.LocationValid`) (`local.RotationValid`)))
  (bind _camera (`/Game/Blueprints/BP_MRPawn.Camera` _pawn))
  (`|ExecutionSequence`
    (:`then_0`
      ;[1 1 1] Grab the Pawn
      (if (not (`KismetSystemLibrary.IsValid` (`self.Pawn`)))
        (bind _asbp_pipes_game_mode (cast `/Game/Blueprints/BP_PipesGameMode` (`GameplayStatics.GetGameMode`)))
        (bind _pawn_2 (`/Game/Blueprints/BP_PipesGameMode.GetPawn` _asbp_pipes_game_mode))
        (set `self.Pawn` _pawn_2)))
    (:`then_1`
      ;[1 1 1] Grab the Camera
      (if (`KismetSystemLibrary.IsValid` _pawn)
        (set `local.CameraPosition` (`SceneComponent.K2_GetComponentLocation` _camera))
        (set `local.CameraForward` (`SceneComponent.GetForwardVector` _camera))
        (set `local.CameraValid` true)))
    (:`then_2`
      ;[1 1 1] Compute the position (which might be overriden by a derived blueprint)
      (if (`local.CameraValid`)
        (set `local.LocationValid` true)
        (bind _location (`self.Compute Position` Initial (`local.CameraPosition`) (`local.CameraForward`)))
        (set `local.Location` _location)))
    (:`then_3`
      ;[1 1 1] Compute the rotation to face the camera from our computed location
      (if (`local.LocationValid`)
        (set `local.Rotation` (`KismetMathLibrary.MakeRotFromXZ` (- (`local.Location`) (`local.CameraPosition`)) (`KismetMathLibrary.Vector_Up`)))
        (set `local.RotationValid` true)))
    (:`then_4`
      ;[1 1 1] Return what we've computed (if anything)
      (return _returnvalue (`KismetMathLibrary.MakeTransform` (`KismetMathLibrary.SelectVector` (`local.Location`) (0.0 0.0 0.0) _returnvalue) (`KismetMathLibrary.SelectRotator` (`local.Rotation`) (struct) _returnvalue))))))

(fn `SetOverride`
  (params (NewOverride :type "/Game/Blueprints/Dialogs/Interface_FollowUser_Override Interface"))
  (set `self.Override` NewOverride)
  (set `self.HasOverride` true))

(fn `UpdatePlacement`
  (bind _location (.location (`Actor.GetTransform` (`self.GetOwner`))))
  (bind (_transformvalid _transform) (`self.ComputePlacement` false))
  (if _transformvalid
    (bind _canlerp (`self.CanLerpTransform`))
    (bind _location_2 (.location _transform))
    (bind _rotation (.rotation _transform))
    (bind _returnvalue (or (not _canlerp) (> (`KismetMathLibrary.VSizeSquared` (- _location _location_2)) 10000.0)))
    (`Actor.K2_SetActorLocationAndRotation` (`self.GetOwner`) (`KismetMathLibrary.SelectVector` _location_2 (`KismetMathLibrary.VLerp` _location _location_2 (`self.UpdateLerpAlpha`)) _returnvalue) (`KismetMathLibrary.SelectRotator` _rotation (`KismetMathLibrary.RLerp` (.rotation (`Actor.GetTransform` (`self.GetOwner`))) _rotation (`self.UpdateLerpAlpha`) true) _returnvalue) false false)))