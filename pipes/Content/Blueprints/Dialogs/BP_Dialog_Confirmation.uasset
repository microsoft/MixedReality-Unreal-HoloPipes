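; Confirmation dialog for the pipe puzzle game, asking Yes/No before actions such as sweeping, moving or recalling the game, export/import, skipping levels or exiting.
; ShowConfirmationDialog stores the confirmation type, adds both buttons through inherited dialog functions and selects the matching prompt, inserting custom text for level skips.
; On dismissal, it broadcasts that type with a confirmed flag, derived from the Yes button's tag, then hides itself.
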(event `self.ReceiveBeginPlay`
  (`parent.ReceiveBeginPlay`)
  (add `self.DialogDismissedDispatcher` (delegate `DialogDismissed`)))

(event `DialogDismissed` :!signature `self.DialogDismissedDispatcher`
  (params (Button :type "/Game/Blueprints/Buttons/BP_Button_Basic Object Reference"))
  (`self.ConfirmationDialogDismissedDispatcher` (`self.CurrentConfirmation`) (== (`/Game/Blueprints/Buttons/BP_Button_Base.Tag` Button) 1))
  (`self.HideConfirmationDialog`))

(fn `HideConfirmationDialog`
  (`self.HideDialog` true))

(fn `ShowConfirmationDialog`
  (params (Confirming :type "/Game/Blueprints/Dialogs/ENUM_Confirmation Enum" :default "NewEnumerator0") (CustomText :type Text))
  (set `self.CurrentConfirmation` Confirming)
  (`self.AddButton` (make `/Game/Blueprints/Dialogs/STRUCT_DialogButton` "Yes" "/Game/UI/Icons/YesIcon.YesIcon" "NewEnumerator0" 1))
  (`self.AddButton` (make `/Game/Blueprints/Dialogs/STRUCT_DialogButton` "No" "/Game/UI/Icons/NoIcon.NoIcon" "NewEnumerator1"))
  (`self.ShowDialog` (select `/Game/Blueprints/Dialogs/ENUM_Confirmation` (`local.Confirming`) :`NewEnumerator1` "Sweeping the level will return all disconnected pipe pieces to the toolbox. \n \nAre you sure you want to sweep?" :`NewEnumerator4` "\"Show Cursor\" enables a crosshair style cursor for each hand to assist with precise targeting. \n \nShow cursors now?" :`NewEnumerator5` "\"Show Labels\" enables per pipe labels on every open pipe end. Instead of connecting matching colors, you can connect matching labels. \n \nShow labels now?" :`NewEnumerator6` "Move the game by pinching with one hand; Move, scale and rotate the game by pinching with both hands. Press or say “Place Game” to return to normal game play. \n \nMove the game now?" :`NewEnumerator7` "\"Recall Game\" returns the game to its default size, orientation and position. \n \nRecall the game now?" :`NewEnumerator8` "Exporting the game captures a snapshot of your progress that can be shared with other players and other devices. \n \nExport your game now?" :`NewEnumerator9` "Your export failed. Would you like to try again?" :`NewEnumerator10` "Importing a game loads a previously exported snapshot, replacing your current progress. This action can't be undone. \n \nImport a game now?" :`NewEnumerator11` "Your import failed. Would you like to try again?" :`NewEnumerator12` "Exit to main menu? \n \nYour progress on this level will be lost." :`NewEnumerator13` (`|FormatText` "Pay 20 stars to skip level {0}? \n \nYou can go back to play it at any time." (`local.CustomText`)))))

(fn `UserConstructionScript`
  (`parent.UserConstructionScript`))