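; BP_Dialog_Error is a world-space error dialog variant that shows a message in a widget which follows the user.
; On BeginPlay it narrows the FollowUser component's distance range so the dialog sits at a set distance.
; ShowErrorDialog casts the TextWidget's widget to WBP_DialogMessage, tints its background dark red, then passes the message to the inherited ShowDialog.
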(event `self.ReceiveBeginPlay`
  (bind _followuser (`self.FollowUser`))
  (`parent.ReceiveBeginPlay`)
  (set `/Game/Blueprints/Dialogs/BP_FollowUser_Component.MinDistance` 40.0 _followuser)
  (set `/Game/Blueprints/Dialogs/BP_FollowUser_Component.MaxDistance` 48.0 _followuser)
  (set `/Game/Blueprints/Dialogs/BP_FollowUser_Component.DesiredDistance` 45.0 _followuser))

(fn `ShowErrorDialog`
  (params (Message :type Text))
  (bind _aswbp_dialog_message (cast `/Game/UI/WBP_DialogMessage` (`WidgetComponent.GetUserWidgetObject` (`self.TextWidget`))))
  (`/Game/UI/WBP_DialogMessage.SetBackgroundColor` _aswbp_dialog_message (struct :`R` 0.45 :`A` 1.0))
  (`self.ShowDialog` (`local.Message`)))

(fn `UserConstructionScript`
  (`parent.UserConstructionScript`))