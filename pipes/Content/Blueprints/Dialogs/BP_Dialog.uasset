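; BP_Dialog is a floating dialog prompt that follows the user and offers a centered row of buttons answerable by click or voice.
; ShowDialog sets the widget message, spawns and attaches BP_Button_Basic actors from queued button data, then places itself via FollowUser with optional sound.
; Voice phrases from the pawn and button clicks both route to Complete, which fires DialogDismissed while visible.
; It also supports hiding, destroying, pausing and resuming.
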(event `self.ReceiveBeginPlay`
  (`SceneComponent.SetVisibility` (`self.DefaultSceneRoot`) false true))

(event `self.ReceiveTick`
  (params (DeltaSeconds :type "Float (single-precision)"))
  (if (`SceneComponent.IsVisible` (`self.DefaultSceneRoot`))
    (`/Game/Blueprints/Dialogs/BP_FollowUser_Component.UpdatePlacement` (`self.FollowUser`))
    (if (not (`self.BoundVoice`))
      (bind _asbp_pipes_game_mode (cast `/Game/Blueprints/BP_PipesGameMode` (`GameplayStatics.GetGameMode`)))
      (bind _pawn (`/Game/Blueprints/BP_PipesGameMode.GetPawn` _asbp_pipes_game_mode))
      (if (`KismetSystemLibrary.IsValid` _pawn)
        (add `/Game/Blueprints/BP_MRPawn.VoiceInputDispatcher` _pawn (delegate `Voice Event`))
        (set `self.BoundVoice` true)))))

(event `Voice Event`
  (params (Phrase :type "/Game/Blueprints/Buttons/ENUM_VoiceInput Enum" :default "NewEnumerator0") (Source :type "/Game/Blueprints/Buttons/Interface_EventSource Interface"))
  (for (_array_element _array_index) (`self.CurrentDialogButtons`)
    (if (== (`.Phrase_9_7ACA52DE4BB8CAD9D8B7ED9F4CDA7432` (break `/Game/Blueprints/Dialogs/STRUCT_DialogButton` _array_element)) Phrase)
      (bind _output (`|GetArrayItem` (`self.BPButtons`) _array_index))
      (if (`/Game/Blueprints/Buttons/BP_Button_Base.Enabled` _output)
        (bind _handled (`self.Complete` _output))
        (if _handled
          (`/Game/Blueprints/Buttons/Interface_EventSource.EventHandled` Source))))))

(event `self.ReceiveDestroyed`
  (`self.DestroyButtons`))

(event `Dialog Button Created`
  (params (Button :type "/Game/Blueprints/Buttons/BP_Button_Base Object Reference"))
  (add `/Game/Blueprints/Buttons/BP_Button_Base.ClickedDispatcher` Button (delegate `OnButtonClicked`)))

(event `OnButtonClicked`
  (params (Source :type "/Game/Blueprints/Buttons/BP_Button_Base Object Reference"))
  (bind _asbp_button_basic (cast `/Game/Blueprints/Buttons/BP_Button_Basic` Source))
  (`self.Complete` _asbp_button_basic))

(fn `AddButton`
  (params (Button :type "/Game/Blueprints/Dialogs/STRUCT_DialogButton Structure"))
  (`KismetArrayLibrary.Array_Add` (`self.NextDialogButtons`) Button))

(fn `Complete`
  (params (Button :type "/Game/Blueprints/Buttons/BP_Button_Basic Object Reference"))
  (returns (Handled :type Boolean))
  (bind _defaultsceneroot (`self.DefaultSceneRoot`))
  (if (and (`KismetSystemLibrary.IsValid` _defaultsceneroot) (`SceneComponent.IsVisible` _defaultsceneroot))
    (`self.DialogDismissedDispatcher` Button)
    (return true)
    (else
      (return false))))

(fn `CreateButtons`
  (locals (NewButton :type "/Game/Blueprints/Buttons/BP_Button_Basic Object Reference") (ButtonsStart :type "Float (double-precision)"))
  (bind _newbutton (`local.NewButton`))
  (bind _currentdialogbuttons (`self.CurrentDialogButtons`))
  (bind _nextdialogbuttons (`self.NextDialogButtons`))
  (set `local.ButtonsStart` (* (`KismetMathLibrary.Conv_IntToDouble` (- (`KismetArrayLibrary.Array_Length` (`self.NextDialogButtons`)) 1)) -0.5 (`self.ButtonCellSize`)))
  (for (_array_element _array_index) (`self.NextDialogButtons`)
    (bind (_text _icon _phrase _tag) (break `/Game/Blueprints/Dialogs/STRUCT_DialogButton` _array_element))
    (bind _returnvalue (`|SpawnActorFromClass` "/Game/Blueprints/Buttons/BP_Button_Basic.BP_Button_Basic_C" (`KismetMathLibrary.MakeTransform` (`KismetMathLibrary.MakeVector` 0.0 (+ (`local.ButtonsStart`) (* _array_index (`self.ButtonCellSize`))) -1.5)) "Undefined" "OverrideRootScale" self _text _icon "Text" false null))
    (bind _output_get (set `local.NewButton` _returnvalue))
    (`self.K2_AttachToActor` _output_get self "None" "KeepRelative" "KeepRelative" "KeepRelative" false)
    (set `/Game/Blueprints/Buttons/BP_Button_Base.Tag` _tag _newbutton)
    (`self.Dialog Button Created` _newbutton)
    (`KismetArrayLibrary.Array_Add` (`self.BPButtons`) _newbutton))
  (`KismetArrayLibrary.Array_Clear` _currentdialogbuttons)
  (`KismetArrayLibrary.Array_Append` _currentdialogbuttons _nextdialogbuttons)
  (`KismetArrayLibrary.Array_Clear` _nextdialogbuttons))

(fn `DestroyButtons`
  (for _array_element (`self.BPButtons`)
    (`self.K2_DestroyActor` _array_element))
  (`KismetArrayLibrary.Array_Clear` (`self.BPButtons`))
  (`KismetArrayLibrary.Array_Clear` (`self.CurrentDialogButtons`)))

(fn `HideDialog`
  (params (Destroy :type Boolean))
  (if (`KismetSystemLibrary.IsValid` self)
    (if (`SceneComponent.IsVisible` (`self.DefaultSceneRoot`))
      (`SceneComponent.SetVisibility` (`self.DefaultSceneRoot`) false true))
    (if (`local.Destroy`)
      (`self.K2_DestroyActor`))))

(fn `PauseDialog`
  (`self.HideDialog` false)
  (set `self.Paused` true))

(fn `ResumeDialog`
  (if (and (`self.Paused`) (not (`self.IsActorBeingDestroyed`)))
    (`self.ShowDialogInternal`)
    (set `self.Paused` false)))

(fn `ShowDialog`
  (params (Prompt :type Text))
  (`|ExecutionSequence`
    (:`then_0`
      (`self.DestroyButtons`)
      (bind _aswbp_dialog_message (cast `/Game/UI/WBP_DialogMessage` (`WidgetComponent.GetUserWidgetObject` (`self.TextWidget`))))
      (`/Game/UI/WBP_DialogMessage.SetMessage` _aswbp_dialog_message (`KismetTextLibrary.Conv_TextToString` (`local.Prompt`)))
      (`WidgetComponent.RequestRedraw` (`self.TextWidget`)))
    (:`then_1`
      (`self.CreateButtons`))
    (:`then_2`
      (`self.ShowDialogInternal`))))

(fn `ShowDialogInternal`
  (`SceneComponent.SetVisibility` (`self.DefaultSceneRoot`) true true)
  (bind (_transformvalid _transform) (`/Game/Blueprints/Dialogs/BP_FollowUser_Component.ComputePlacement` (`self.FollowUser`) (`self.ShowSetsInitialPlacement`)))
  (if _transformvalid
    (`SceneComponent.K2_SetWorldTransform` (`self.DefaultSceneRoot`) _transform false false)
    (if (`self.ShowPlaysSound`)
      (`GameplayStatics.PlaySoundAtLocation` "/Game/Sounds/HoloPipe_Dialog.HoloPipe_Dialog" (`SceneComponent.K2_GetComponentLocation` (`self.DefaultSceneRoot`)) (struct) 1.0 1.0 0.0 null null null))))

(fn `UserConstructionScript`)