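; BP_Pipe is the visual and audio actor for one piece in a grid-based pipe puzzle.
; On initialization it builds runtime meshes and dynamic materials for its pipe type, with fixed-piece caps and translucent-or-blocked proxy handling.
; Timelines fade class colors and grow toolbox pieces in.
; Events play drag/rotate sounds, spawn weld effects from a connection bitmask, and manage a class label and hand/gaze focus debug cube.
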(event `self.ReceiveBeginPlay`
  (`|ExecutionSequence`
    (:`then_0`
      (bind (_direction _alpha) (`Timeline|Timeline Color` :!via `Stop`)
        (:`Update`
          _)
        (:`Finished`
          _))
      (`MaterialInstanceDynamic.SetVectorParameterValue` (`self.MainMaterial`) "Color" (`KismetMathLibrary.LinearColorLerp` (`self.ColorPrevious`) (`self.ColorNext`) _alpha)))
    (:`then_1`
      (bind (_direction_2 _scale) (`Timeline|Timeline Grow In` :!via `Stop`)
        (:`Update`
          _)
        (:`Finished`
          _))
      (`SceneComponent.SetRelativeScale3D` (`self.DefaultSceneRoot`) (`KismetMathLibrary.MakeVector` _scale _scale _scale)))))

(event `self.OnPipeInitializationComplete`
  (`self.HandleInitializationComplete`))

(event `self.OnPipeClassChanged`
  (params (newClass :type Integer))
  (`self.SetPipeColor` newClass true))

(event `self.OnFixedChanged`
  (`self.SetPipeColor` (`self.PipeClass`)))

(event `self.OnInteractionEvent`
  (params (InteractionEvent :type "EInteractionEvent Enum" :default "DragStarted"))
  (bind _returnvalue (`SceneComponent.K2_GetComponentLocation` (`self.DefaultSceneRoot`)))
  (switch `EInteractionEvent` InteractionEvent
    (:`DragStarted`
      (`GameplayStatics.PlaySoundAtLocation` "/Game/Sounds/HoloPipe_Grab.HoloPipe_Grab" _returnvalue (struct) 0.5 1.0 0.0 null null null :!label _label))
    (:`DragFinished`
      (`GameplayStatics.PlaySoundAtLocation` "/Game/Sounds/HoloPipe_Release.HoloPipe_Release" _returnvalue (struct) 2.0 1.0 0.0 null null null :!label _label_2))
    (:`DragFinishedBlocked`
      (`GameplayStatics.PlaySoundAtLocation` "/Game/Sounds/HoloPipe_PIpe_Blocked.HoloPipe_PIpe_Blocked" _returnvalue (struct) 1.0 1.0 0.0 null null null)
      (`self.HandleNewConnections` :!label _label_3))
    (:`DragFinishedConnected`
      (`GameplayStatics.PlaySoundAtLocation` "/Game/Sounds/HoloPipe_Pipe_Connect.HoloPipe_Pipe_Connect" _returnvalue (struct) 0.5 0.5 0.13 null null null :!label _label_4)
      (goto _label_3))
    (:`RotateStarted`
      (goto _label))
    (:`RotateFinished`
      (goto _label_2))
    (:`RotateFinishedConnected`
      (goto _label_4))))

(event `self.OnProxyTypeChanged`
  (params (proxyType :type "EPipeProxyType Enum" :default "None"))
  (`SceneComponent.SetVisibility` (`self.DefaultSceneRoot`) (`|EnumInequality` proxyType "ProxyBlocked") true))

(event `self.OnShowLabelChanged`
  (params (show :type Boolean))
  (`self.HandleShowLabel` show))

(event `self.ReceiveDestroyed`
  (bind _pipelabel (`self.PipeLabel`))
  (if (`KismetSystemLibrary.IsValid` _pipelabel)
    (`self.K2_DestroyActor` _pipelabel)))

(event `self.OnFocusStageChanged`
  (params (stage :type "EFocusStage Enum" :default "None"))
  (`self.HandleFocusStageChanged` stage))

(fn `CreateBlock`
  (bind _returnvalue (`AddComponent|NODE_AddStaticMeshComponent-9` :`RelativeTransform` (`KismetMathLibrary.MakeTransform` (0.0 0.0 0.0) (struct) (0.15 0.15 0.15))))
  (`StaticMeshComponent.SetStaticMesh` _returnvalue "/Engine/EngineMeshes/Cube.Cube")
  (`PrimitiveComponent.SetMaterial` _returnvalue 0 "/Game/Materials/MAT_MetalScreen.MAT_MetalScreen"))

(fn `CreateCaps`
  (bind _pipetype (`self.PipeType`))
  (if (and (`self.PipeFixed`) (not (`self.InToolbox`)))
    (`self.CreateEndsMaterial` true)
    (`self.CreateRightCap`)
    (if (or (`|EnumEquality` _pipetype "Straight") (`|EnumEquality` _pipetype "Junction"))
      (`self.CreateLeftCap`))
    (if (or (`|EnumEquality` _pipetype "Corner") (`|EnumEquality` _pipetype "Junction"))
      (`self.CreateTopCap`))))

(fn `CreateCornerPipe`
  (bind _returnvalue (`AddComponent|NODE_AddStaticMeshComponent-1` :`RelativeTransform` (`KismetMathLibrary.MakeTransform` (20.0 0.0 0.0) (struct :`Pitch` 90.0))))
  (`StaticMeshComponent.SetStaticMesh` _returnvalue "/Game/Pipes/Meshes/Elbow_geo.Elbow_geo")
  (`PrimitiveComponent.SetMaterial` _returnvalue 0 (`self.MainMaterial`)))

(fn `CreateEndPipe`
  (`self.CreateStraightPipe`)
  (`|ExecutionSequence`
    (:`then_0`
      (bind _returnvalue (`AddComponent|NODE_AddStaticMeshComponent-4` :`RelativeTransform` (`KismetMathLibrary.MakeTransform` (-5.8 0.0 0.0))))
      (`StaticMeshComponent.SetStaticMesh` _returnvalue "/Game/Pipes/Meshes/EndFlange_geo.EndFlange_geo")
      (`self.CreateEndsMaterial` false)
      (`PrimitiveComponent.SetMaterial` _returnvalue 0 (`self.EndsMaterial`)))
    (:`then_1`
      (bind _returnvalue_2 (`AddComponent|NODE_AddStaticMeshComponent-11` :`RelativeTransform` (`KismetMathLibrary.MakeTransform` (-16.0 0.0 0.0) (`KismetMathLibrary.MakeRotator` (select `bool` (>= (`KismetMathLibrary.RandomFloatInRange` 0.0 1.0) 0.5) :`false` 180.0) 0.0 (select `bool` (>= (`KismetMathLibrary.RandomFloatInRange` 0.0 1.0) 0.5) :`false` 180.0)))))
      (`StaticMeshComponent.SetStaticMesh` _returnvalue_2 "/Game/Pipes/Meshes/Wall_geo.Wall_geo"))))

(fn `CreateEndsMaterial`
  (params (ForValve :type Boolean))
  (bind _returnvalue (`KismetMaterialLibrary.CreateDynamicMaterialInstance` (select `bool` ForValve :`false` "/Game/Pipes/Materials/MI_EndFlange.MI_EndFlange" :`true` "/Game/Pipes/Materials/MI_Valve.MI_Valve" :!type "MaterialInterface Object Reference")))
  (set `self.EndsMaterial` _returnvalue))

(fn `CreateLeftCap`
  (bind _returnvalue (`AddComponent|NODE_AddStaticMeshComponent-7` :`RelativeTransform` (`KismetMathLibrary.MakeTransform` (-19.0 0.0 0.0) (struct) (0.4 0.8 0.8))))
  (`StaticMeshComponent.SetStaticMesh` _returnvalue "/Game/Pipes/Meshes/Coupler_geo.Coupler_geo")
  (`PrimitiveComponent.SetMaterial` _returnvalue 0 (`self.EndsMaterial`)))

(fn `CreateMainMaterial`
  (bind _returnvalue (`KismetMaterialLibrary.CreateDynamicMaterialInstance` (select `EPipeProxyType` (`self.ProxyType`) :`None` "/Game/Pipes/Materials/MI_Pipes.MI_Pipes" :`ProxyReady` "/Game/Pipes/Materials/MI_Proxy.MI_Proxy" :`ProxyBlocked` "/Game/Pipes/Materials/MI_Proxy.MI_Proxy" :!type "MaterialInterface Object Reference")))
  (set `self.MainMaterial` _returnvalue))

(fn `CreatePipe`
  (bind _pipetype (`self.GetCurrentPipeType`))
  (switch `EPipeType` _pipetype
    (:`Start`
      (`self.CreateStartPipe`))
    (:`End`
      (`self.CreateEndPipe`))
    (:`Straight`
      (`self.CreateStraightPipe`)
      (`self.CreateCaps` :!label _label))
    (:`Corner`
      (`self.CreateCornerPipe`)
      (goto _label))
    (:`Junction`
      (`self.CreateTPipe`)
      (goto _label))
    (:`Block`
      (`self.CreateBlock`))))

(fn `CreateRightCap`
  (bind _returnvalue (`AddComponent|NODE_AddStaticMeshComponent-6` :`RelativeTransform` (`KismetMathLibrary.MakeTransform` (19.26 0.0 0.0) (struct) (0.4 0.8 0.8))))
  (`StaticMeshComponent.SetStaticMesh` _returnvalue "/Game/Pipes/Meshes/Coupler_geo.Coupler_geo")
  (`PrimitiveComponent.SetMaterial` _returnvalue 0 (`self.EndsMaterial`)))

(fn `CreateStartPipe`
  (`self.CreateStraightPipe`)
  (`|ExecutionSequence`
    (:`then_0`
      (bind _returnvalue (`AddComponent|NODE_AddStaticMeshComponent-3` :`RelativeTransform` (`KismetMathLibrary.MakeTransform` (-5.3 0.0 0.0) (struct) (0.8 0.8 0.8))))
      (`StaticMeshComponent.SetStaticMesh` _returnvalue "/Game/Pipes/Meshes/Valve_geo.Valve_geo")
      (`self.CreateEndsMaterial` true)
      (`PrimitiveComponent.SetMaterial` _returnvalue 0 (`self.EndsMaterial`)))
    (:`then_1`
      (bind _returnvalue_2 (`AddComponent|NODE_AddStaticMeshComponent-12` :`RelativeTransform` (`KismetMathLibrary.MakeTransform` (-16.0 0.0 0.0) (`KismetMathLibrary.MakeRotator` (select `bool` (>= (`KismetMathLibrary.RandomFloatInRange` 0.0 1.0) 0.5) :`false` 180.0) 0.0 (select `bool` (>= (`KismetMathLibrary.RandomFloatInRange` 0.0 1.0) 0.5) :`false` 180.0)))))
      (`StaticMeshComponent.SetStaticMesh` _returnvalue_2 "/Game/Pipes/Meshes/Wall_geo.Wall_geo"))))

(fn `CreateStraightPipe`
  (bind _returnvalue (`AddComponent|NODE_AddStaticMeshComponent-2` :`bManualAttachment` true :`RelativeTransform` (`KismetMathLibrary.MakeTransform` (0.0 0.0 0.0) (`KismetMathLibrary.MakeRotator` 0.0 0.0 (`KismetMathLibrary.Conv_IntToDouble` (* (`KismetMathLibrary.RandomInteger` 12) 30))))))
  (`StaticMeshComponent.SetStaticMesh` _returnvalue "/Game/Pipes/Meshes/Pipe_geo.Pipe_geo")
  (`PrimitiveComponent.SetMaterial` _returnvalue 0 (`self.MainMaterial`))
  (bind _returnvalue_2 (`AddComponent|NODE_AddSceneComponent-1` :`RelativeTransform` (`KismetMathLibrary.MakeTransform` (20.0 0.0 0.0) (struct :`Pitch` 90.0) (1.0 1.0 0.8))))
  (`SceneComponent.K2_AttachToComponent` _returnvalue _returnvalue_2 "None" "KeepRelative" "KeepRelative" "KeepRelative" false))

(fn `CreateTopCap`
  (bind _returnvalue (`AddComponent|NODE_AddStaticMeshComponent-8` :`RelativeTransform` (`KismetMathLibrary.MakeTransform` (0.0 0.0 19.0) (struct :`Pitch` 90.0) (0.5 0.8 0.8))))
  (`StaticMeshComponent.SetStaticMesh` _returnvalue "/Game/Pipes/Meshes/Coupler_geo.Coupler_geo")
  (`PrimitiveComponent.SetMaterial` _returnvalue 0 (`self.EndsMaterial`)))

(fn `CreateTPipe`
  (bind _returnvalue (`AddComponent|NODE_AddStaticMeshComponent-0` :`RelativeTransform` (`KismetMathLibrary.MakeTransform` (0.0 0.0 0.0))))
  (`StaticMeshComponent.SetStaticMesh` _returnvalue "/Game/Pipes/Meshes/TJunction_geo.TJunction_geo")
  (`PrimitiveComponent.SetMaterial` _returnvalue 0 (`self.MainMaterial`)))

(fn `GetCurrentPipeClass`
  (returns (PipeClass :type Integer))
  (return (`self.PipeClass`)))

(fn `GetCurrentPipeType`
  (returns (PipeType :type "EPipeType Enum"))
  (return (`self.PipeType`)))

(fn `HandleFocusStageChanged`
  (params (Stage :type "EFocusStage Enum" :default "None"))
  (bind _gazefocuscube (`self.GazeFocusCube`))
  (bind _gazefocuscube_2 (`self.GazeFocusCube`))
  (if (`|EnumInequality` Stage)
    (if (not (`KismetSystemLibrary.IsValid` (`self.GazeFocusCube`)))
      (bind _returnvalue (`AddComponent|NODE_AddStaticMeshComponent-10` :`bManualAttachment` true :`RelativeTransform` (`KismetMathLibrary.MakeTransform` (0.0 0.0 0.0) (struct) (0.3 0.3 0.3))))
      (bind _output_get (set `self.GazeFocusCube` _returnvalue))
      (`StaticMeshComponent.SetStaticMesh` _output_get "/Engine/BasicShapes/Cube.Cube")
      (`SceneComponent.K2_AttachToComponent` _output_get (`Actor.RootComponent` (`self.GetOwner`)) "None" "KeepRelative" "KeepRelative" "KeepRelative" true)
      (bind _returnvalue_2 (`PrimitiveComponent.CreateDynamicMaterialInstance` _output_get 0 "/Game/Materials/Utility/MAT_DebugGrid_Inst.MAT_DebugGrid_Inst" "None"))
      (set `self.GazeFocusCubeMaterial` _returnvalue_2))
    (`SceneComponent.SetVisibility` _gazefocuscube_2 true false)
    (`SceneComponent.K2_SetRelativeLocation` _gazefocuscube_2 (.location (`SceneComponent.GetRelativeTransform` (`self.DefaultSceneRoot`))) false false)
    (`MaterialInstanceDynamic.SetVectorParameterValue` (`self.GazeFocusCubeMaterial`) "Color" (select `EFocusStage` (`local.Stage`) :`None` (struct :`A` 1.0) :`HandOnly` (struct :`R` 0.1 :`G` 0.1 :`B` 0.1 :`A` 1.0) :`HandAndGaze` (struct :`R` 0.4 :`B` 0.4 :`A` 1.0) :`HandAndGazeAndDistance` (struct :`G` 0.5 :`B` 0.5 :`A` 1.0) :!type "LinearColor Structure"))
    (elif (`KismetSystemLibrary.IsValid` _gazefocuscube)
      (`SceneComponent.SetVisibility` _gazefocuscube false false))))

(fn `HandleInitializationComplete`
  (`self.CreateMainMaterial`)
  (`self.CreatePipe`)
  (bind _pipeclass (`self.GetCurrentPipeClass`))
  (`self.SetPipeColor` _pipeclass)
  (if (`|EnumInequality` (`self.ProxyType`))
    (`self.SetActorRelativeScale3D` (0.85 0.85 0.85))
    (elif (`self.InToolbox`)
      (`TimelineComponent.PlayFromStart` (`self.Timeline Grow In`)))))

(fn `HandleNewConnection`
  (params (Candidate :type Integer) (Offset :type "Vector Structure") (Rotation :type "Rotator Structure"))
  (if (!= (`KismetMathLibrary.And_IntInt` Candidate (`self.PipeConnections`)) 0)
    (bind _asbp_pipes_game_mode (cast `/Game/Blueprints/BP_PipesGameMode` (`GameplayStatics.GetGameMode`)))
    (`GameplayStatics.SpawnEmitterAttached` "/Game/Particles/P_WeldRings.P_WeldRings" (`Actor.RootComponent` (`PPipesGameMode.PipeGrid` _asbp_pipes_game_mode)) "None" (+ (`SceneComponent.RelativeLocation` (`self.DefaultSceneRoot`)) (`local.Offset`)) (`local.Rotation`) (1.0 1.0 1.0) "SnapToTargetIncludingScale")))

(fn `HandleNewConnections`
  (`self.HandleNewConnection` (`|BitmaskLiteral` 4) (0.0 -20.0 0.0) (struct :`Roll` 90.0))
  (`self.HandleNewConnection` (`|BitmaskLiteral` 1) (0.0 20.0 0.0) (struct :`Roll` 90.0))
  (`self.HandleNewConnection` (`|BitmaskLiteral` 2) (20.0 0.0 0.0) (struct :`Pitch` 90.0))
  (`self.HandleNewConnection` (`|BitmaskLiteral` 8) (-20.0 0.0 0.0) (struct :`Pitch` 90.0))
  (`self.HandleNewConnection` (`|BitmaskLiteral` 16) (0.0 0.0 20.0))
  (`self.HandleNewConnection` (`|BitmaskLiteral` 32) (0.0 0.0 -20.0)))

(fn `HandleShowLabel`
  (params (Show :type Boolean))
  (bind _pipelabel (`self.PipeLabel`))
  (bind _returnvalue (`KismetSystemLibrary.IsValid` _pipelabel))
  (if Show
    (if (not _returnvalue)
      (bind _returnvalue_2 (`|SpawnActorFromClass` "/Game/Blueprints/Pipes/BP_PipeLabel.BP_PipeLabel_C" (`KismetMathLibrary.MakeTransform` (0.0 0.0 0.0)) "AlwaysSpawn" "OverrideRootScale" self null))
      (bind _output_get (set `self.PipeLabel` _returnvalue_2))
      (`self.K2_AttachToActor` _output_get self "None" "KeepRelative" "KeepWorld" "KeepRelative" true))
    (`/Game/Blueprints/Pipes/BP_PipeLabel.SetLabel` _output_get (`.Label_11_9CBD3E4F4654AED736858083426C4AE6` (break `/Game/Blueprints/Pipes/STRUCT_PipeColor` (`|GetArrayItem` (`self.PipeColors`) (`self.PipeClass`)))))
    (elif _returnvalue
      (`self.K2_DestroyActor` _pipelabel))))

(fn `SetPipeColor`
  (params (ColorIndex :type Integer) (Fade :type Boolean))
  (bind _pipecolors (`self.PipeColors`))
  (bind _pipelabel (`self.PipeLabel`))
  (bind _endsmaterial (`self.EndsMaterial`))
  (bind _returnvalue (* (`self.ColorNext`) (`KismetMathLibrary.SelectFloat` 0.1 1.0 (and (== ColorIndex 0) (`self.PipeFixed`)))))
  (bind (_output_name _output_color _output_label) (break `/Game/Blueprints/Pipes/STRUCT_PipeColor` (`|GetArrayItem` _pipecolors (`KismetMathLibrary.Clamp` ColorIndex 0 (- (`KismetArrayLibrary.Array_Length` _pipecolors) 1)))))
  (if (`|EnumEquality` (`self.ProxyType`))
    (`|ExecutionSequence`
      (:`then_0`
        (set `self.ColorNext` (`KismetMathLibrary.Conv_ColorToLinearColor` _output_color))
        (if (`KismetSystemLibrary.IsValid` _pipelabel)
          (`/Game/Blueprints/Pipes/BP_PipeLabel.SetLabel` _pipelabel _output_label)))
      (:`then_1`
        (if Fade
          (bind _returnvalue_2 (`MaterialInstanceDynamic.K2_GetVectorParameterValue` (`self.MainMaterial`) "Color"))
          (set `self.ColorPrevious` _returnvalue_2)
          (`TimelineComponent.PlayFromStart` (`self.Timeline Color`))
          (else
            (`MaterialInstanceDynamic.SetVectorParameterValue` (`self.MainMaterial`) "Color" _returnvalue)
            ;[0.1667 1 0.2621] The start/end segments have a different material than the pipes
            (if (`KismetSystemLibrary.IsValid` _endsmaterial)
              (`MaterialInstanceDynamic.SetVectorParameterValue` _endsmaterial "Color" _returnvalue))))))))

(fn `UserConstructionScript`)