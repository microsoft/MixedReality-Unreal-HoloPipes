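; BP_PipeLabel is a floating text label for the pipes game that turns to face the player's camera.
; On BeginPlay it feeds the text component's texture and mask into a dynamic masked material on a plane, and SetLabel updates that text.
; Each Tick it aims the root at the camera of the pawn cached from BP_PipesGameMode and scales the plane with the root, clamped to a minimum world size.
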(event `self.ReceiveBeginPlay`
  (bind _textplanetext (`self.TextPlaneText`))
  (`/Game/Blueprints/DynamicText/BP_DynamicTextWithMask.SetTextureSize` _textplanetext 44 44 true)
  (bind _returnvalue (`PrimitiveComponent.CreateDynamicMaterialInstance` (`self.TextPlane`) 0 "/Game/Materials/MAT_TextWithMask.MAT_TextWithMask" "None"))
  (`MaterialInstanceDynamic.SetTextureParameterValue` _returnvalue "Text" (`/Game/Blueprints/DynamicText/BP_DynamicTextWithMask.Texture` _textplanetext))
  (`MaterialInstanceDynamic.SetTextureParameterValue` _returnvalue "Mask" (`/Game/Blueprints/DynamicText/BP_DynamicTextWithMask.Mask` _textplanetext)))

(event `self.ReceiveTick`
  (params (DeltaSeconds :type "Float (single-precision)"))
  (bind _returnvalue (`KismetMathLibrary.FMax` (* (.x (`SceneComponent.K2_GetComponentScale` (`self.DefaultSceneRoot`))) (`self.DefaultRelativeScale`)) (`self.MinWorldScale`)))
  (if (`KismetSystemLibrary.IsValid` (`self.Pawn`))
    (`SceneComponent.K2_SetWorldRotation` (`self.DefaultSceneRoot`) (`KismetMathLibrary.MakeRotFromXZ` (- (`SceneComponent.K2_GetComponentLocation` (`/Game/Blueprints/BP_MRPawn.Camera` (`self.Pawn`))) (`SceneComponent.K2_GetComponentLocation` (`self.DefaultSceneRoot`))) (`KismetMathLibrary.Vector_Up`)) false false :!label _label)
    (`SceneComponent.SetWorldScale3D` (`self.TextPlane`) (`KismetMathLibrary.MakeVector` _returnvalue _returnvalue _returnvalue))
    (else
      (bind _asbp_pipes_game_mode (cast `/Game/Blueprints/BP_PipesGameMode` (`GameplayStatics.GetGameMode`)))
      (bind _pawn (`/Game/Blueprints/BP_PipesGameMode.GetPawn` _asbp_pipes_game_mode))
      (bind _output_get (set `self.Pawn` _pawn))
      (if (`KismetSystemLibrary.IsValid` _output_get)
        (goto _label)))))

(fn `SetLabel`
  (params (Label :type String))
  (`/Game/Blueprints/DynamicText/BP_DynamicTextWithMask.SetTextureText` (`self.TextPlaneText`) (`KismetTextLibrary.Conv_StringToText` Label)))

(fn `UserConstructionScript`)