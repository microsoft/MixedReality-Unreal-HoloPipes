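; BP_TargetCursor is a reticle cursor that marks a targeting location and shows whether the pointer is pinched.
; UpdateState takes a dirty state, moves the cursor to its location and recolors the dynamic reticle material shared by its planes, brighter in the Ready phase.
; Tick shows it only while a phase is active and the pawn, fetched lazily from BP_PipesGameMode and cached, has no interactable focused.
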(event `self.ReceiveBeginPlay`
  (bind _returnvalue (`PrimitiveComponent.CreateDynamicMaterialInstance` (`self.Plane2`) 0 "/Game/Materials/MAT_Reticle.MAT_Reticle" "None"))
  (bind _output_get (set `self.CursorMaterial` _returnvalue))
  (`PrimitiveComponent.SetMaterial` (`self.Plane3`) 0 _output_get)
  (`PrimitiveComponent.SetMaterial` (`self.Plane1`) 0 _output_get))

(event `self.ReceiveTick`
  (params (DeltaSeconds :type "Float (single-precision)"))
  (bind _targetcursor (`self.TargetCursor`))
  (if (`self.VisibleDesired`)
    (if (`KismetSystemLibrary.IsValid` (`self.Pawn`))
      (if (`KismetSystemLibrary.IsValid` (stale _output_get)) :!label _label
        (bind _focused (`/Game/Blueprints/BP_MRPawn.AnyInteractableFocused` (stale _output_get)))
        (if (not _focused)
          (`SceneComponent.SetVisibility` _targetcursor true true)
          (else
            (`SceneComponent.SetVisibility` _targetcursor false true :!label _label_2)))
        (else
          (goto _label_2)))
      (else
        (bind _asbp_pipes_game_mode (cast `/Game/Blueprints/BP_PipesGameMode` (`GameplayStatics.GetGameMode`))
          (:`then`
            (bind _pawn (`/Game/Blueprints/BP_PipesGameMode.GetPawn` _asbp_pipes_game_mode))
            (bind _output_get (set `self.Pawn` _pawn))
            (goto _label))
          (:`CastFailed`
            (goto _label_2)))))
    (else
      (goto _label_2))))

(fn `UpdateState`
  (params (State :type "SimpleCursorState Structure"))
  (locals (CursorTargetColor :type "LinearColor Structure"))
  (bind (_phase _location _dirty) (break `SimpleCursorState` State))
  (bind _cursormaterial (`self.CursorMaterial`))
  (bind _pinched (`self.Pinched`))
  (if _dirty
    (set `self.Pinched` (`|EnumEquality` _phase "Ready"))
    (bind _output_get (set `self.VisibleDesired` (`|EnumInequality` _phase)))
    (if _output_get
      (`SceneComponent.K2_SetRelativeLocation` (`self.TargetCursor`) _location false false)
      (`MaterialInstanceDynamic.SetVectorParameterValue` _cursormaterial "Color" (`KismetMathLibrary.SelectColor` (struct :`R` 0.7 :`G` 0.7 :`A` 1.0) (struct :`R` 0.2 :`G` 0.2 :`A` 1.0) _pinched))
      (`MaterialInstanceDynamic.SetVectorParameterValue` _cursormaterial "BorderColor" (`KismetMathLibrary.SelectColor` (struct :`R` 1.0 :`G` 1.0 :`B` 1.0 :`A` 1.0) (struct) _pinched)))))

(fn `UserConstructionScript`)