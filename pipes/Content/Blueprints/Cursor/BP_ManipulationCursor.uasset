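; Manipulation cursor that shows translate and rotate feedback as a highlighted cell, a rotation handle and yaw, pitch and roll hints.
; UpdateCursor applies dirty parts of a hand cursor state, setting visibility, transforms and phase colors through dynamic materials.
; The handle orients to the active axis and scales in by timeline when it changes, unless suppressed.
; UpdateHints combines both phases to color all axis hints, isolating the active axis when Ready.
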(event `self.ReceiveBeginPlay`
  (bind _returnvalue (`PrimitiveComponent.CreateDynamicMaterialInstance` (`self.CellCursor`) 0 "/Game/Materials/MAT_Highlight_Inst.MAT_Highlight_Inst" "None"))
  (set `self.CellCursorMaterial` _returnvalue)
  (bind _returnvalue_2 (`PrimitiveComponent.CreateDynamicMaterialInstance` (`self.HandleCursorHandle`) 0 "/Game/Materials/MAT_BasicUnlit_Inst.MAT_BasicUnlit_Inst" "None"))
  (bind _output_get (set `self.RotateCursorMaterial` _returnvalue_2))
  (`PrimitiveComponent.SetMaterial` (`self.HandleCursorShaft1`) 0 _output_get)
  (`PrimitiveComponent.SetMaterial` (`self.HandleCursorShaft2`) 0 _output_get)
  (`self.InitializeHints`)
  (`self.UpdateCursor` (make `CursorStateHand` (struct :`Location` (0.0 0.0 0.0)) (make `SimpleCursorState` "None" (0.0 0.0 0.0) true) (make `RotateCursorState` "None" (0.0 0.0 0.0) "None" (struct) true)))
  (bind (_direction _progress) (`Timeline|ShowRotateHandleTimeline` :!via `Stop`)
    (:`Update`
      _)
    (:`Finished`
      _))
  (`self.UpdateHandleCursor` _progress))

(fn `HideHandleCursor`
  (`SceneComponent.SetVisibility` (`self.HandleCursor`) false true))

(fn `InitializeHints`
  (`self.InitializeHintsForAxis` (`self.PitchRoot`) (`self.PitchHint`) "Pitch")
  (`self.InitializeHintsForAxis` (`self.YawRoot`) (`self.YawHint`) "Yaw")
  (`self.InitializeHintsForAxis` (`self.RollRoot`) (`self.RollHint`) "Roll"))

(fn `InitializeHintsForAxis`
  (params (Parent :type "SceneComponent Object Reference") (Color :type "LinearColor Structure") (Axis :type "EInteractionAxis Enum" :default "None"))
  (locals (HintMaterial :type "MaterialInstanceDynamic Object Reference"))
  (bind _returnvalue (select `EInteractionAxis` Axis :`Yaw` (`self.YawHint`) :`Pitch` (`self.PitchHint`) :`Roll` (`self.RollHint`)))
  (bind _returnvalue_2 (`KismetMaterialLibrary.CreateDynamicMaterialInstance` "/Game/Materials/MAT_BasicUnlit.MAT_BasicUnlit"))
  (`MaterialInstanceDynamic.SetVectorParameterValue` _returnvalue_2 "Color" Color)
  (`KismetArrayLibrary.Array_Add` (`self.Hints`) (make `/Game/Blueprints/Cursor/STRUCT_CursorAxis` Axis Parent _returnvalue_2 _returnvalue _returnvalue (`self.CellPending`) (select `EInteractionAxis` Axis :`Yaw` (`self.YawActive`) :`Pitch` (`self.PitchActive`) :`Roll` (`self.RollActive`))))
  (for _array_element (`SceneComponent.GetChildrenComponents` Parent false)
    (bind _asstatic_mesh_component (cast `StaticMeshComponent` _array_element))
    (`PrimitiveComponent.SetMaterial` _asstatic_mesh_component 0 _returnvalue_2)
    (`SceneComponent.SetVisibility` _asstatic_mesh_component false false)))

(fn `UpdateCursor`
  (params (State :type "CursorStateHand Structure"))
  (locals (RotatePending :type Boolean) (HandleRotator :type "Rotator Structure") (AxisChanged :type Boolean) (SuppressAxisChangeAnimation :type Boolean))
  (bind (_target _translate _rotate) (break `CursorStateHand` State))
  (bind _cellcursor (`self.CellCursor`))
  (bind _cellcursormaterial (`self.CellCursorMaterial`))
  (bind _showrotatehandletimeline (`self.ShowRotateHandleTimeline`))
  (bind (_phase _location _dirty) (break `SimpleCursorState` _translate))
  (bind (_phase_2 _location_2 _axis _axisrotations _dirty_2 _suppresschangeanimation) (break `RotateCursorState` _rotate))
  (bind _returnvalue (`KismetMathLibrary.SelectFloat` 1.0 -1.0 (`|EnumEquality` _phase_2)))
  (bind _returnvalue_2 (> (.y _location_2) 0.0))
  (`|ExecutionSequence`
    (:`then_0`
      (if _dirty
        (if (`|EnumEquality` _phase)
          (`SceneComponent.SetVisibility` _cellcursor false false)
          (else
            (`MaterialInstanceDynamic.SetVectorParameterValue` _cellcursormaterial "Color" (select `EInteractionPhase` _phase :`Visible` (`self.CellVisible`) :`Pending` (`self.CellPending`) :`Blocked` (`self.CellBlocked`) :`Ready` (`self.CellReady`)))
            (`MaterialInstanceDynamic.SetScalarParameterValue` _cellcursormaterial "Solid" (select `EInteractionPhase` _phase :`None` 1.0 :`Visible` _returnvalue :`Pending` _returnvalue :`Blocked` 1.0 :`Ready` 1.0))
            (`SceneComponent.SetVisibility` _cellcursor true false)
            (`SceneComponent.K2_SetRelativeLocation` (`self.ManipulationCursor`) _location false false)))))
    (:`then_1`
      (if _dirty_2
        (set `local.SuppressAxisChangeAnimation` _suppresschangeanimation)
        (set `local.AxisChanged` (or (`|EnumInequality` _axis (`self.CurrentAxis`)) (!= _location_2 (`SceneComponent.RelativeLocation` (`self.HandleCursor`)) :`ErrorTolerance` 5.0)))
        (`SceneComponent.K2_SetRelativeLocation` (`self.HandleCursor`) _location_2 false false)
        (set `self.CurrentAxis` _axis)
        (`SceneComponent.K2_SetRelativeRotation` (`self.ManipulationCursor`) _axisrotations false false)
        (switch `EInteractionPhase` _phase_2
          (:`None`
            (`TimelineComponent.Stop` (`self.ShowRotateHandleTimeline`) :!label _label)
            (set `self.CurrentAxis` "None")
            (`self.HideHandleCursor`))
          (:`Visible`
            (goto _label))
          (:`Pending`
            (set `local.RotatePending` true)
            (if (`|EnumEquality` _axis) :!label _label_2
              (goto _label)
              (else
                (`SceneComponent.K2_SetRelativeRotation` (`self.HandleCursorInner`) (select `EInteractionAxis` _axis :`Yaw` (struct :`Yaw` -90.0 :`Roll` 90.0) :`Roll` (struct :`Yaw` 90.0) :!type "Rotator Structure") false false)
                (`SceneComponent.K2_SetRelativeRotation` (`self.HandleCursor`) (`KismetMathLibrary.MakeRotator` (.x (* (* (select `EInteractionAxis` _axis :`Yaw` (0.0 0.0 1.0) :`Pitch` (0.0 -1.0 0.0) :`Roll` (1.0 0.0 0.0) :!type "Vector Structure") (`KismetMathLibrary.DegAcos` (`KismetMathLibrary.Dot_VectorVector` (`KismetMathLibrary.Normal` _location_2) (select `EInteractionAxis` _axis :`Yaw` (1.0 0.0 1.0) :`Pitch` (0.0 0.0 1.0) :`Roll` (0.0 0.0 1.0) :!type "Vector Structure")))) (`KismetMathLibrary.SelectFloat` 1.0 -1.0 (select `EInteractionAxis` (`self.CurrentAxis`) :`Yaw` _returnvalue_2 :`Pitch` (> (.x _location_2) 0.0) :`Roll` _returnvalue_2)))) (.y (* (* (select `EInteractionAxis` _axis :`Yaw` (0.0 0.0 1.0) :`Pitch` (0.0 -1.0 0.0) :`Roll` (1.0 0.0 0.0) :!type "Vector Structure") (`KismetMathLibrary.DegAcos` (`KismetMathLibrary.Dot_VectorVector` (`KismetMathLibrary.Normal` _location_2) (select `EInteractionAxis` _axis :`Yaw` (1.0 0.0 1.0) :`Pitch` (0.0 0.0 1.0) :`Roll` (0.0 0.0 1.0) :!type "Vector Structure")))) (`KismetMathLibrary.SelectFloat` 1.0 -1.0 (select `EInteractionAxis` (`self.CurrentAxis`) :`Yaw` _returnvalue_2 :`Pitch` (> (.x _location_2) 0.0) :`Roll` _returnvalue_2)))) (.z (* (* (select `EInteractionAxis` _axis :`Yaw` (0.0 0.0 1.0) :`Pitch` (0.0 -1.0 0.0) :`Roll` (1.0 0.0 0.0) :!type "Vector Structure") (`KismetMathLibrary.DegAcos` (`KismetMathLibrary.Dot_VectorVector` (`KismetMathLibrary.Normal` _location_2) (select `EInteractionAxis` _axis :`Yaw` (1.0 0.0 1.0) :`Pitch` (0.0 0.0 1.0) :`Roll` (0.0 0.0 1.0) :!type "Vector Structure")))) (`KismetMathLibrary.SelectFloat` 1.0 -1.0 (select `EInteractionAxis` (`self.CurrentAxis`) :`Yaw` _returnvalue_2 :`Pitch` (> (.x _location_2) 0.0) :`Roll` _returnvalue_2))))) false false)
                (`MaterialInstanceDynamic.SetVectorParameterValue` (`self.RotateCursorMaterial`) "Color" (`KismetMathLibrary.SelectColor` (select `EInteractionAxis` _axis :`Yaw` (`self.YawHint`) :`Pitch` (`self.PitchHint`) :`Roll` (`self.RollHint`)) (select `EInteractionAxis` _axis :`Yaw` (`self.YawActive`) :`Pitch` (`self.PitchActive`) :`Roll` (`self.RollActive`)) (`local.RotatePending`)))
                (`MaterialInstanceDynamic.SetVectorParameterValue` (`self.CellCursorMaterial`) "Color" (`KismetMathLibrary.SelectColor` (`self.CellVisible`) (select `EInteractionAxis` _axis :`Yaw` (`self.YawHint`) :`Pitch` (`self.PitchHint`) :`Roll` (`self.RollHint`)) (`local.RotatePending`)))
                (if (`local.AxisChanged`)
                  (if (`local.SuppressAxisChangeAnimation`)
                    (`TimelineComponent.Stop` _showrotatehandletimeline)
                    (`self.UpdateHandleCursor` 1.0)
                    (else
                      (`TimelineComponent.PlayFromStart` _showrotatehandletimeline)))))))
          (:`Blocked`
            (goto _label))
          (:`Ready`
            (goto _label_2)))))
    (:`then_2`
      (if (or _dirty _dirty_2)
        (`self.UpdateHints` _phase _phase_2 _axis)))))

(fn `UpdateHandleCursor`
  (params (Progress :type "Float (double-precision)"))
  (`SceneComponent.SetRelativeScale3D` (`self.HandleCursor`) (`KismetMathLibrary.MakeVector` Progress Progress Progress))
  (`SceneComponent.SetVisibility` (`self.HandleCursor`) true true))

(fn `UpdateHints`
  (params (TranslatePhase :type "EInteractionPhase Enum" :default "None") (RotatePhase :type "EInteractionPhase Enum" :default "None") (RotateAxis :type "EInteractionAxis Enum" :default "None"))
  (locals (CommonHintsPhase :type "EInteractionPhase Enum") (ShowHints :type Boolean) (DragPending :type Boolean))
  (bind _commonhintsphase (`local.CommonHintsPhase`))
  (bind _rotateaxis (`local.RotateAxis`))
  (`|ExecutionSequence`
    (:`then_0`
      (switch `EInteractionPhase` TranslatePhase
        (:`Visible`
          _)
        (:`Pending`
          (set `local.DragPending` true)))
      (set `local.ShowHints` true))
    (:`then_1`
      (if (`local.ShowHints`)
        (switch `EInteractionPhase` (`local.RotatePhase`)
          (:`None`
            (set `local.ShowHints` false))
          (:`Visible`
            (if (`local.DragPending`)
              (set `local.CommonHintsPhase` "Blocked")
              (else
                (set `local.CommonHintsPhase` "Pending" :!label _label))))
          (:`Pending`
            (goto _label))
          (:`Blocked`
            (if (`local.DragPending`)
              (set `local.CommonHintsPhase` "Blocked")
              (else
                (set `local.CommonHintsPhase` "Visible"))))
          (:`Ready`
            (set `local.CommonHintsPhase` "Ready")))))
    (:`then_2`
      (if (`local.ShowHints`)
        (if (`|EnumEquality` (`local.CommonHintsPhase`) "Ready")
          (`self.UpdateHintsInner` (select `bool` (`|EnumEquality` _rotateaxis "Yaw") :`true` "Ready" :!type "EInteractionPhase Enum") (select `bool` (`|EnumEquality` _rotateaxis "Pitch") :`true` "Ready" :!type "EInteractionPhase Enum") (select `bool` (`|EnumEquality` _rotateaxis "Roll") :`true` "Ready" :!type "EInteractionPhase Enum"))
          (else
            (`self.UpdateHintsInner` _commonhintsphase _commonhintsphase _commonhintsphase :!label _label_2)))
        (else
          (set `local.CommonHintsPhase` "None")
          (goto _label_2))))))

(fn `UpdateHintsInner`
  (params (YawPhase :type "EInteractionPhase Enum" :default "None") (PitchPhase :type "EInteractionPhase Enum" :default "None") (RollPhase :type "EInteractionPhase Enum" :default "None"))
  (for _array_element (`self.Hints`)
    (bind (_axis _root _material _visiblecolor _pendingcolor _blockedcolor _readycolor) (break `/Game/Blueprints/Cursor/STRUCT_CursorAxis` _array_element))
    (bind _returnvalue (select `EInteractionAxis` _axis :`Yaw` YawPhase :`Pitch` PitchPhase :`Roll` RollPhase))
    (`SceneComponent.SetVisibility` _root (`|EnumInequality` _returnvalue) true)
    (`MaterialInstanceDynamic.SetVectorParameterValue` _material "Color" (select `EInteractionPhase` _returnvalue :`Visible` _visiblecolor :`Pending` _pendingcolor :`Blocked` _blockedcolor :`Ready` _readycolor))))

(fn `UserConstructionScript`)