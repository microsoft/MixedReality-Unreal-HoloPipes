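; BP_ConnectionsCursor is a cursor that shows connection directions on six sides, apparently for pipe placement.
; All six side meshes share one dynamic material, and SetCursorState toggles each side's visibility from a Directions bitmask.
; Pending tints them grey and Ready green, while None and Blocked hide all; a red tint branch is unconnected.
; An orientation sound plays when directions change while the cursor stays Ready and rotation is Ready.
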(event `self.ReceiveBeginPlay`
  (bind _returnvalue (`PrimitiveComponent.CreateDynamicMaterialInstance` (`self.Front`) 0 "/Game/Materials/MAT_BasicUnlit_Inst.MAT_BasicUnlit_Inst" "None"))
  (bind _output_get (set `self.CursorMaterial` _returnvalue))
  (`PrimitiveComponent.SetMaterial` (`self.Back`) 0 _output_get)
  (`PrimitiveComponent.SetMaterial` (`self.Left`) 0 _output_get)
  (`PrimitiveComponent.SetMaterial` (`self.Right`) 0 _output_get)
  (`PrimitiveComponent.SetMaterial` (`self.Top`) 0 _output_get)
  (`PrimitiveComponent.SetMaterial` (`self.Bottom`) 0 _output_get)
  (`self.ClearCursorState`))

(fn `ClearCursorState`
  (`self.SetCursorState` 0))

(fn `SetCursorState`
  (params (Directions :type Integer) (Phase :type "EInteractionPhase Enum" :default "None") (RotatePhase :type "EInteractionPhase Enum" :default "None"))
  (bind _cursormaterial (`self.CursorMaterial`))
  (`|ExecutionSequence`
    (:`then_0`
      (switch `EInteractionPhase` Phase
        (:`None`
          (`SceneComponent.SetVisibility` (`self.Front`) false false :!label _label)
          (`SceneComponent.SetVisibility` (`self.Back`) false false)
          (`SceneComponent.SetVisibility` (`self.Left`) false false)
          (`SceneComponent.SetVisibility` (`self.Right`) false false)
          (`SceneComponent.SetVisibility` (`self.Top`) false false)
          (`SceneComponent.SetVisibility` (`self.Bottom`) false false))
        (:`Pending`
          (`MaterialInstanceDynamic.SetVectorParameterValue` _cursormaterial "Color" (struct :`R` 0.2 :`G` 0.2 :`B` 0.2 :`A` 1.0))
          (`SceneComponent.SetVisibility` (`self.Front`) (!= (`KismetMathLibrary.And_IntInt` Directions (`|BitmaskLiteral` 2)) 0) false :!label _label_2)
          (`SceneComponent.SetVisibility` (`self.Back`) (!= (`KismetMathLibrary.And_IntInt` Directions (`|BitmaskLiteral` 8)) 0) false)
          (`SceneComponent.SetVisibility` (`self.Left`) (!= (`KismetMathLibrary.And_IntInt` Directions (`|BitmaskLiteral` 4)) 0) false)
          (`SceneComponent.SetVisibility` (`self.Right`) (!= (`KismetMathLibrary.And_IntInt` Directions (`|BitmaskLiteral` 1)) 0) false)
          (`SceneComponent.SetVisibility` (`self.Top`) (!= (`KismetMathLibrary.And_IntInt` Directions (`|BitmaskLiteral` 16)) 0) false)
          (`SceneComponent.SetVisibility` (`self.Bottom`) (!= (`KismetMathLibrary.And_IntInt` Directions (`|BitmaskLiteral` 32)) 0) false))
        (:`Blocked`
          (goto _label))
        (:`Ready`
          (`MaterialInstanceDynamic.SetVectorParameterValue` _cursormaterial "Color" (struct :`R` 0.1 :`G` 0.5 :`B` 0.1 :`A` 1.0))
          (goto _label_2))))
    (:`then_1`
      (if (and (!= Directions (`self.LastDirections`)) (`|EnumEquality` Phase "Ready") (`|EnumEquality` (`self.LastPhase`) "Ready") (`|EnumEquality` RotatePhase "Ready"))
        (`GameplayStatics.PlaySoundAtLocation` "/Game/Sounds/HoloPipe_Orientation.HoloPipe_Orientation" (`SceneComponent.K2_GetComponentLocation` (`self.DefaultSceneRoot`)) (struct) 0.25 1.0 0.0 null null null)))
    (:`then_2`
      (set `self.LastDirections` Directions)
      (set `self.LastPhase` Phase))))

(fn `UserConstructionScript`)