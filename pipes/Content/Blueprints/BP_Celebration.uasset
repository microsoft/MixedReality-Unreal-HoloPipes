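; BP_Celebration is a world-space level-complete celebration in the pipes game, revealing awarded stars on a widget, then destroying itself.
; It positions itself at the pipe root from BP_PipesGameMode and smoothly turns to face the pawn's camera each tick.
; Chained function-name timers drive the sequence: scale-in timeline with confetti, per-star sounds and count updates, extra confetti on a fourth star, then scale-out.
; Event dispatchers signal start and completion.
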(event `self.ReceiveBeginPlay`
  (bind _asbp_pipes_game_mode (cast `/Game/Blueprints/BP_PipesGameMode` (`GameplayStatics.GetGameMode`)))
  (bind (_transformvalid _transform) (`/Game/Blueprints/BP_PipesGameMode.ComputePipeRootTransform` _asbp_pipes_game_mode))
  (if _transformvalid
    (`SceneComponent.K2_SetWorldLocation` (`self.Celebration`) (.location _transform) false false)
    (bind _aswbp_celebration (cast `/Game/UI/WBP_Celebration` (`WidgetComponent.GetUserWidgetObject` (`self.CelebrationWidget`))))
    (`/Game/UI/WBP_Celebration.InitializeCelebration` _aswbp_celebration (`self.LevelCompleted`) (`self.MaxStarsAvailable`))
    (`SceneComponent.SetWorldScale3D` (`self.WidgetContainer`) (0.0 0.0 0.0))
    (`KismetSystemLibrary.K2_SetTimer` self "StartHandler" (`self.StartDelay`))
    (bind (_direction _scale) (`Timeline|RevealWidgetTimeline` :!via `Stop`)
      (:`Update`
        _)
      (:`Finished`
        _))
    (`SceneComponent.SetWorldScale3D` (`self.WidgetContainer`) (`KismetMathLibrary.MakeVector` _scale _scale _scale))))

(event `self.ReceiveTick`
  (params (DeltaSeconds :type "Float (single-precision)"))
  (bind (_valid _rotator) (`self.ComputeRotation`))
  (if _valid
    (if (`self.RotationInitialized`)
      (`SceneComponent.K2_SetWorldRotation` (`self.Celebration`) (`KismetMathLibrary.RLerp` (`SceneComponent.K2_GetComponentRotation` (`self.Celebration`)) _rotator 0.05 true) false false)
      (else
        (`SceneComponent.K2_SetWorldRotation` (`self.Celebration`) _rotator false false)
        (set `self.RotationInitialized` true)))))

(fn `CompleteHandler`
  (`self.CompleteEventDispatcher`)
  (`self.K2_DestroyActor`))

(fn `ComputeRotation`
  (returns (Valid :type Boolean) (Rotator :type "Rotator Structure"))
  (locals (CameraPosition :type "Vector Structure") (CameraValid :type Boolean) (Rotation :type "Rotator Structure") (RotationValid :type Boolean))
  (bind _rotationvalid (`local.RotationValid`))
  (bind _pawn (`self.Pawn`))
  (`|ExecutionSequence`
    (:`then_0`
      ;[1 1 1] Grab the Pawn
      (if (not (`KismetSystemLibrary.IsValid` (`self.Pawn`)))
        (bind _asbp_pipes_game_mode (cast `/Game/Blueprints/BP_PipesGameMode` (`GameplayStatics.GetGameMode`)))
        (bind _pawn_2 (`/Game/Blueprints/BP_PipesGameMode.GetPawn` _asbp_pipes_game_mode))
        (set `self.Pawn` _pawn_2)))
    (:`then_1`
      ;[1 1 1] Grab the Camera
      (if (`KismetSystemLibrary.IsValid` _pawn)
        (set `local.CameraPosition` (`SceneComponent.K2_GetComponentLocation` (`/Game/Blueprints/BP_MRPawn.Camera` _pawn)))
        (set `local.CameraValid` true)))
    (:`then_2`
      ;[1 1 1] Compute the rotation to face the camera from our current location
      (if (`local.CameraValid`)
        (set `local.Rotation` (`KismetMathLibrary.MakeRotFromXZ` (- (`local.CameraPosition`) (`SceneComponent.K2_GetComponentLocation` (`self.Celebration`))) (`KismetMathLibrary.Vector_Up`)))
        (set `local.RotationValid` true)))
    (:`then_3`
      ;[1 1 1] Return what we've computed (if anything)
      (return _rotationvalid (`KismetMathLibrary.SelectRotator` (`local.Rotation`) (struct) _rotationvalid)))))

(fn `HideHandler`
  (`TimelineComponent.ReverseFromEnd` (`self.RevealWidgetTimeline`)))

(fn `ProgressHandler`
  (bind _starsreported (`self.StarsReported`))
  (bind _starsreported_2 (`self.StarsReported`))
  (if (< (`self.StarsReported`) (`self.StarsAwarded`))
    (`GameplayStatics.PlaySound2D` (select `int` _starsreported :`0` "/Game/Sounds/HoloPipe_Star_01.HoloPipe_Star_01" :`1` "/Game/Sounds/HoloPipe_Star_02.HoloPipe_Star_02" :`2` "/Game/Sounds/HoloPipe_Star_03.HoloPipe_Star_03" :`3` "/Game/Sounds/HoloPipe_Star_04.HoloPipe_Star_04" :!type "SoundBase Object Reference") (select `int` _starsreported :`0` 0.85 :`1` 0.85 :`2` 0.85 :`3` 1.5 :!type "Float (single-precision)") 1.0 0.0 null null)
    (`/Engine/EditorBlueprintResources/StandardMacros.IncrementInt` _starsreported_2
      (:`  `
        (bind _aswbp_celebration (cast `/Game/UI/WBP_Celebration` (`WidgetComponent.GetUserWidgetObject` (`self.CelebrationWidget`))))
        (`/Game/UI/WBP_Celebration.SetCount` _aswbp_celebration _starsreported_2)
        (`KismetSystemLibrary.K2_SetTimer` self "ProgressHandler" (select `bool` (and (== (`self.StarsReported`) 3) (== (`self.StarsAwarded`) 4)) :`false` 0.75 :`true` 1.25 :!type "Float (single-precision)"))
        (if (== (`self.StarsReported`) 4)
          (`self.StartConfetti`))))
    (else
      (`KismetSystemLibrary.K2_SetTimer` self "HideHandler" 1.5)
      (`KismetSystemLibrary.K2_SetTimer` self "CompleteHandler" 2.0))))

(fn `StartConfetti`
  (bind _returnvalue (`SceneComponent.K2_GetComponentLocation` (`self.Celebration`)))
  (`GameplayStatics.PlaySoundAtLocation` "/Game/Sounds/HoloPipe_Confetti.HoloPipe_Confetti" _returnvalue (struct) 1.0 1.0 0.0 null "/Game/Sounds/CelebrationConcurrency.CelebrationConcurrency" null)
  (`GameplayStatics.SpawnEmitterAtLocation` "/Game/Particles/P_Confetti.P_Confetti" _returnvalue))

(fn `StartHandler`
  (`self.StartingEventDispatcher`)
  (`self.StartConfetti`)
  (`TimelineComponent.PlayFromStart` (`self.RevealWidgetTimeline`))
  (`KismetSystemLibrary.K2_SetTimer` self "ProgressHandler" 1.0))

(fn `UserConstructionScript`)