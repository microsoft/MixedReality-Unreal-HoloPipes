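; Base push button, registered with the pawn as an interactable, that is physically pressed by a focus point.
; Each tick, the focus point in button-local space, which must enter from the front, drives the face's stroke and dynamic material colors.
; Full stroke engages and captures pawn focus; release while focused fires Click, toggling Checked for checkable buttons and calling dispatchers.
; Child-prefixed functions handle face setup and checked visuals.
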(event `self.ReceiveBeginPlay`
  (`self.ChildInitializeFace`)
  (`self.UpdateButtonState`)
  (`self.ChildHandleCheckedChange`))

(event `self.ReceiveTick`
  (params (DeltaSeconds :type "Float (single-precision)"))
  (`|ExecutionSequence`
    (:`then_0`
      (if (not (`self.Registered`))
        (bind _asbp_pipes_game_mode (cast `/Game/Blueprints/BP_PipesGameMode` (`GameplayStatics.GetGameMode`)))
        (bind _pawn (`/Game/Blueprints/BP_PipesGameMode.GetPawn` _asbp_pipes_game_mode))
        (if (`KismetSystemLibrary.IsValid` _pawn)
          (`/Game/Blueprints/BP_MRPawn.AddInteractable` _pawn self)
          (set `self.Registered` true))))
    (:`then_1`
      (`self.UpdateButtonState`))
    (:`then_2`
      (if (`self.ScheduleEngage`)
        (set `self.ScheduleEngage` false)
        (`self.HandleEngage`)))
    (:`then_3`
      (if (`self.ScheduleActivate`)
        (set `self.ScheduleActivate` false)
        (`self.HandleActivate`)))))

(event `self.ReceiveEndPlay`
  (params (EndPlayReason :type "EEndPlayReason Enum" :default "Destroyed"))
  (bind _returnvalue (`GameplayStatics.GetGameMode`))
  (if (`KismetSystemLibrary.IsValid` _returnvalue)
    (bind _asbp_pipes_game_mode (cast `/Game/Blueprints/BP_PipesGameMode` _returnvalue))
    (bind _pawn (`/Game/Blueprints/BP_PipesGameMode.GetPawn` _asbp_pipes_game_mode))
    (if (`KismetSystemLibrary.IsValid` _pawn)
      (`/Game/Blueprints/BP_MRPawn.RemoveInteractable` _pawn self))))

(event `/Game/Blueprints/Buttons/Interface_Interactable.UpdateFocusPoint`
  (params (Focus :type "/Game/Blueprints/Buttons/ENUM_Focus Enum" :default "NewEnumerator0") (Location :type "Vector Structure"))
  (set `self.ReportedFocusPoint` Location)
  (set `self.ReportedFocusPointValid` (`|EnumEquality` "NewEnumerator0" Focus))
  (if (and (`self.Engaged`) (`|EnumEquality` Focus "NewEnumerator2"))
    (set `self.Engaged` false)))

(fn `ChildHandleCheckedChange`
  (`MaterialInstanceDynamic.SetScalarParameterValue` (`self.ButtonFaceMaterial`) "Checked" (`KismetMathLibrary.SelectFloat` 1.0 -1.0 (`self.Checked`))))

(fn `ChildInitializeFace`
  (bind _returnvalue (`PrimitiveComponent.CreateDynamicMaterialInstance` (`self.ButtonFace`) 0 "/Game/Materials/MAT_Button.MAT_Button" "None"))
  (set `self.ButtonFaceMaterial` _returnvalue))

(fn `Click`
  (if (`self.CanCheck`)
    (bind _output_get (set `self.Checked` (not (`self.Checked`))))
    (`self.CheckedChangedDispatcher` _output_get self))
  (`self.ClickedDispatcher` self))

(fn `HandleActivate`
  (if (`self.Engaged`)
    (`self.UpdateEngaged` false)
    (`self.PlayButtonSound` false)
    (if (`self.Focused`)
      (`self.Click`))))

(fn `HandleEngage`
  (if (not (`self.Engaged`))
    (`self.UpdateEngaged` true)
    (`self.PlayButtonSound` true)))

(fn `PlayButtonSound`
  (params (Press :type Boolean))
  (`GameplayStatics.PlaySoundAtLocation` "/Game/Sounds/HoloPipe_Select.HoloPipe_Select" (`self.K2_GetActorLocation`) (struct) 2.0 (`KismetMathLibrary.SelectFloat` 1.0 1.1 Press) 0.0 null null null))

(fn `QueryFocusPoint`
  (params (FocusPoint :type "Vector Structure"))
  (returns (Type :type "/Game/Blueprints/Buttons/ENUM_FocusPointType Enum") (Cursor :type "/Game/Blueprints/Buttons/ENUM_CursorType Enum") (Point :type "Vector Structure") (Normal :type "Vector Structure"))
  (bind _returnvalue (`SceneComponent.K2_GetComponentToWorld` (`self.ButtonContainer`)))
  (bind _returnvalue_2 (/ (`self.Width`) 2.0))
  (bind _returnvalue_3 (* -1.0 _returnvalue_2))
  (bind _x (.x (.location (`SceneComponent.GetRelativeTransform` (`self.ButtonContainer`)))))
  (bind _y (.y (`KismetMathLibrary.TransformLocation` (`KismetMathLibrary.InvertTransform` (`SceneComponent.K2_GetComponentToWorld` (`self.ButtonContainer`))) FocusPoint)))
  (bind _z (.z (`KismetMathLibrary.TransformLocation` (`KismetMathLibrary.InvertTransform` (`SceneComponent.K2_GetComponentToWorld` (`self.ButtonContainer`))) FocusPoint)))
  (bind _returnvalue_4 (`KismetMathLibrary.FClamp` _z _returnvalue_3 _returnvalue_2))
  (bind _returnvalue_5 (`KismetMathLibrary.FClamp` _y _returnvalue_3 _returnvalue_2))
  (if (and (`SceneComponent.IsVisible` (`self.ButtonContainer`)) (`self.Enabled`))
    (return (select `bool` (or (and (== _returnvalue_5 _y) (== _returnvalue_4 _z) (or (< (.x (`KismetMathLibrary.TransformLocation` (`KismetMathLibrary.InvertTransform` (`SceneComponent.K2_GetComponentToWorld` (`self.ButtonContainer`))) FocusPoint)) 0.0) (`self.Focused`))) (`self.Engaged`)) :`false` "NewEnumerator2" :`true` "NewEnumerator1" :!type "/Game/Blueprints/Buttons/ENUM_FocusPointType Enum") "NewEnumerator0" (`KismetMathLibrary.TransformLocation` _returnvalue (`KismetMathLibrary.SelectVector` (`KismetMathLibrary.MakeVector` _x _y _z) (`KismetMathLibrary.MakeVector` _x _returnvalue_5 _returnvalue_4) (`self.Engaged`))) (`KismetMathLibrary.TransformDirection` _returnvalue (`KismetMathLibrary.Vector_Backward`)))
    (else
      (return "NewEnumerator0" "NewEnumerator0" (0.0 0.0 0.0) (0.0 0.0 0.0)))))

(fn `UpdateButtonState`
  (bind _returnvalue (`KismetMathLibrary.SelectColor` (`self.ForegroundColor`) (`self.DisabledForegroundColor`) (`self.Enabled`)))
  (bind _returnvalue_2 (`KismetMathLibrary.SelectColor` (`KismetMathLibrary.SelectColor` (`self.CheckedColor`) (`self.DefaultColor`) (`self.Checked`)) (`self.DisabledColor`) (`self.Enabled`)))
  (bind _returnvalue_3 (`KismetMathLibrary.SelectColor` _returnvalue_2 (`KismetMathLibrary.LinearColorLerp` (`KismetMathLibrary.LinearColorLerp` _returnvalue_2 (`self.FocusedModifierColor`) 0.25) (`self.PressedColor`) (`self.Stroke`)) (not (`self.Focused`))))
  (if (not (`self.IsActorBeingDestroyed`))
    (`self.UpdateFocus`)
    (`self.UpdateStroke`)
    (if (not (`KismetMathLibrary.LinearColor_IsNearEqual` (`self.LastBackColor`) _returnvalue_3 0.001))
      (bind _output_get (set `self.LastBackColor` _returnvalue_3))
      (`MaterialInstanceDynamic.SetVectorParameterValue` (`self.ButtonFaceMaterial`) "Color" _output_get))
    (if (not (`KismetMathLibrary.LinearColor_IsNearEqual` (`self.LastForeColor`) _returnvalue 0.001))
      (set `self.LastForeColor` _returnvalue)
      (`MaterialInstanceDynamic.SetVectorParameterValue` (`self.ButtonFaceMaterial`) "ForegroundColor" _returnvalue))
    (if (and (`self.CanCheck`) (!= (`self.Checked`) (`self.WasChecked`)))
      (set `self.WasChecked` (`self.Checked`))
      (`self.ChildHandleCheckedChange`))))

(fn `UpdateEngaged`
  (params (Engage :type Boolean))
  (locals (Pawn :type "/Game/Blueprints/BP_MRPawn Object Reference"))
  (bind _pawn (`local.Pawn`))
  (if (!= Engage (`self.Engaged`))
    (bind _asbp_pipes_game_mode (cast `/Game/Blueprints/BP_PipesGameMode` (`GameplayStatics.GetGameMode`)))
    (bind _pawn_2 (`/Game/Blueprints/BP_PipesGameMode.GetPawn` _asbp_pipes_game_mode))
    (bind _output_get (set `local.Pawn` _pawn_2))
    (if (`KismetSystemLibrary.IsValid` _output_get)
      (if (`local.Engage`)
        (set `self.Engaged` true)
        (`/Game/Blueprints/BP_MRPawn.CaptureFocus` _pawn self "AnyHand")
        (else
          (set `self.Engaged` false)
          (`/Game/Blueprints/BP_MRPawn.ReleaseFocus` _pawn self))))))

(fn `UpdateFocus`
  (bind _returnvalue (/ (`KismetMathLibrary.SelectFloat` (`self.EngagedWidth`) (`self.Width`) (`self.Engaged`)) 2.0))
  (bind _returnvalue_2 (* _returnvalue -1.0))
  (bind _x (.x (`KismetMathLibrary.TransformLocation` (`KismetMathLibrary.InvertTransform` (`SceneComponent.K2_GetComponentToWorld` (`self.ButtonRoot`))) (`self.ReportedFocusPoint`))))
  (if (and (`SceneComponent.IsVisible` (`self.ButtonContainer`)) (`self.Enabled`) (`self.ReportedFocusPointValid`))
    (bind _output_get (set `self.CurrentFocusedPosition` _x))
    (set `self.Focused` (and (and (`KismetMathLibrary.InRange_FloatFloat` _x (* (`self.MaxFocusLength`) -1.0) (`self.MaxBackGutter`)) (`KismetMathLibrary.InRange_FloatFloat` (.y (`KismetMathLibrary.TransformLocation` (`KismetMathLibrary.InvertTransform` (`SceneComponent.K2_GetComponentToWorld` (`self.ButtonRoot`))) (`self.ReportedFocusPoint`))) _returnvalue_2 _returnvalue) (`KismetMathLibrary.InRange_FloatFloat` (.z (`KismetMathLibrary.TransformLocation` (`KismetMathLibrary.InvertTransform` (`SceneComponent.K2_GetComponentToWorld` (`self.ButtonRoot`))) (`self.ReportedFocusPoint`))) _returnvalue_2 _returnvalue)) (or (< _output_get 0.0) (`self.Focused`))))
    (else
      (set `self.Focused` false)
      (`self.UpdateEngaged` false))))

(fn `UpdateStroke`
  (locals (FaceX :type "Float (double-precision)"))
  (bind _currentfocusedposition (`self.CurrentFocusedPosition`))
  (if (`self.Enabled`)
    (if (`self.Focused`)
      (if (< _currentfocusedposition 0.0)
        (set `local.FaceX` 0.0 :!label _label)
        (set `self.Stroke` 0.0)
        (set `self.ScheduleActivate` (`self.Engaged`))
        (elif (> (`self.MaxStrokeLength`) _currentfocusedposition)
          (bind _output_get (set `local.FaceX` _currentfocusedposition))
          (set `self.Stroke` (/ _output_get (`self.MaxStrokeLength`)))
          (else
            (set `local.FaceX` (`self.MaxStrokeLength`) :!label _label_2)
            (set `self.Stroke` 1.0)
            (set `self.ScheduleEngage` (and (not (`self.Engaged`)) (`self.Enabled`))))))
      (else
        (goto _label)))
    (else
      (goto _label_2)))
  (`SceneComponent.K2_SetRelativeLocation` (`self.ButtonContainer`) (`KismetMathLibrary.MakeVector` (`local.FaceX`)) false false))

(fn `UserConstructionScript`)