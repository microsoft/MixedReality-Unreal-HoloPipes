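; BP_Button_Basic is a button Blueprint that shows an icon and a text label on its face material.
; Its setters feed the icon to the Face parameter and render the label through DynamicText into a texture for the Text parameter.
; It overrides parent hooks to apply both on face initialization and, on checked changes, redraw the text, using the checked label when one is set.
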(fn `ChildHandleCheckedChange`
  (`parent.ChildHandleCheckedChange`)
  (`/Game/Blueprints/DynamicText/BP_DynamicText.SetTextureText` (`self.DynamicText`) (select `bool` (and (`self.Checked`) (not (`KismetTextLibrary.TextIsEmpty` (`self.CheckedButtonText`)))) :`false` (`self.ButtonText`) :`true` (`self.CheckedButtonText`))))

(fn `ChildInitializeFace`
  (`parent.ChildInitializeFace`)
  (`self.SetButtonIcon` (`self.ButtonIcon`))
  (`self.SetButtonText` (`self.ButtonText`)))

(fn `GetButtonText`
  (returns (Text :type Text))
  (return (`self.ButtonText`)))

(fn `SetButtonIcon`
  (params (Icon :type "Texture2D Object Reference"))
  (bind _output_get (set `self.ButtonIcon` Icon))
  (`MaterialInstanceDynamic.SetTextureParameterValue` (`self.ButtonFaceMaterial`) "Face" _output_get))

(fn `SetButtonText`
  (params (Text :type Text))
  (bind _dynamictext (`self.DynamicText`))
  (bind _output_get (set `self.ButtonText` Text))
  (`/Game/Blueprints/DynamicText/BP_DynamicText.SetTextureText` _dynamictext _output_get)
  (`MaterialInstanceDynamic.SetTextureParameterValue` (`self.ButtonFaceMaterial`) "Text" (`/Game/Blueprints/DynamicText/BP_DynamicText.Texture` _dynamictext)))

(fn `UserConstructionScript`
  (`parent.UserConstructionScript`))