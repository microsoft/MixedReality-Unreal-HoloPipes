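; A short-lived floating text tooltip, placed along the player's gaze on spawn and named as voice-related.
; On BeginPlay it sets the position from the pawn's gaze with a height offset, then renders the text into a masked dynamic material on a plane.
; A timeline animates the plane's scale and vertical offset, then destroys the actor on finish.
; Every tick the tooltip rotates upright to face the gaze origin.
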(event `self.ReceiveBeginPlay`
  (bind _tooltipplanetext (`self.TooltipPlaneText`))
  (bind _tooltipplane (`self.TooltipPlane`))
  (bind (_origin _direction) (`self.GetGazeState`))
  (bind _output_get (set `self.InitialPosition` (`KismetMathLibrary.MakeVector` (.x (+ _origin (* _direction (`self.InitialDistance`)))) (.y (+ _origin (* _direction (`self.InitialDistance`)))) (+ (.z (+ _origin (* _direction (`self.InitialDistance`)))) (`self.InitialZOffset`)))))
  (`SceneComponent.K2_SetWorldLocation` (`self.Tooltip`) _output_get false false)
  (set `self.InitialScale` (`SceneComponent.RelativeScale3D` _tooltipplane))
  (`SceneComponent.SetRelativeScale3D` _tooltipplane (0.0 0.0 0.0))
  (`/Game/Blueprints/DynamicText/BP_DynamicTextWithMask.SetTextureSize` _tooltipplanetext 246 44 false)
  (`/Game/Blueprints/DynamicText/BP_DynamicTextWithMask.SetTextureForeColor` _tooltipplanetext (struct :`R` 0.6 :`G` 0.6 :`B` 0.6 :`A` 1.0) false)
  (`/Game/Blueprints/DynamicText/BP_DynamicTextWithMask.SetTextureText` _tooltipplanetext (`self.Text`))
  (bind _returnvalue (`PrimitiveComponent.CreateDynamicMaterialInstance` (`self.TooltipPlane`) 0 "/Game/Materials/MAT_TextWithMask.MAT_TextWithMask" "None"))
  (`MaterialInstanceDynamic.SetTextureParameterValue` _returnvalue "Text" (`/Game/Blueprints/DynamicText/BP_DynamicTextWithMask.Texture` _tooltipplanetext))
  (`MaterialInstanceDynamic.SetTextureParameterValue` _returnvalue "Mask" (`/Game/Blueprints/DynamicText/BP_DynamicTextWithMask.Mask` _tooltipplanetext))
  (bind (_direction_2 _zoffset _scale) (`Timeline|LifetimeTimeline`)
    (:`Update`
      (`SceneComponent.K2_SetWorldLocation` (`self.Tooltip`) (`KismetMathLibrary.MakeVector` (.x (`self.InitialPosition`)) (.y (`self.InitialPosition`)) (+ (.z (`self.InitialPosition`)) _zoffset)) false false)
      (`SceneComponent.SetRelativeScale3D` (`self.TooltipPlane`) (* (`self.InitialScale`) _scale)))
    (:`Finished`
      (`self.K2_DestroyActor`))))

(event `self.ReceiveTick`
  (params (DeltaSeconds :type "Float (single-precision)"))
  (bind _origin (`self.GetGazeState`))
  (`SceneComponent.K2_SetWorldRotation` (`self.Tooltip`) (`KismetMathLibrary.MakeRotFromXZ` (- _origin (`SceneComponent.K2_GetComponentLocation` (`self.Tooltip`))) (`KismetMathLibrary.Vector_Up`)) false false))

(fn `GetGazeState`
  (returns (Origin :type "Vector Structure") (Direction :type "Vector Structure"))
  (bind _asbp_pipes_game_mode (cast `/Game/Blueprints/BP_PipesGameMode` (`GameplayStatics.GetGameMode`)))
  (bind _pawn (`/Game/Blueprints/BP_PipesGameMode.GetPawn` _asbp_pipes_game_mode))
  (if (`KismetSystemLibrary.IsValid` _pawn)
    (bind (_origin _direction) (`/Game/Blueprints/BP_MRPawn.DetectGazeState` _pawn))
    (return _origin _direction)
    (else
      (return (0.0 0.0 0.0) (1.0 0.0 0.0)))))

(fn `UserConstructionScript`)