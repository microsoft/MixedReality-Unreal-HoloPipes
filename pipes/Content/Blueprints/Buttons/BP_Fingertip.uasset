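; Hand-tracked fingertip cursor that selects a focus target for near interaction and shows a ring with an optional scroll arrow.
; Each tick derives interaction and render points from two joints of the hand.
; Externally called functions rank candidates by containment and observer or finger distance, filter by angle and range, then commit or clear focus.
; The ring shrinks and aligns to the target as it nears, pinning near the surface when penetration would hide it.
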(event `self.ReceiveBeginPlay`
  (bind _returnvalue (`PrimitiveComponent.CreateDynamicMaterialInstance` (`self.RingPlane`) 0 "/Game/Materials/MAT_Ring.MAT_Ring" "None"))
  (bind _output_get (set `self.RingMaterial` _returnvalue))
  (`MaterialInstanceDynamic.SetScalarParameterValue` _output_get "BorderThickness" (`self.BorderThickness`))
  (`MaterialInstanceDynamic.SetScalarParameterValue` _output_get "OuterRadius" (`self.MaxRadius`))
  (`MaterialInstanceDynamic.SetScalarParameterValue` _output_get "Thickness" (`self.Thickness`))
  (bind _returnvalue_2 (`PrimitiveComponent.CreateDynamicMaterialInstance` (`self.ArrowPlane`) 0 "/Game/Materials/MAT_Scroll.MAT_Scroll" "None"))
  (set `self.ArrowMaterial` _returnvalue_2))

(event `self.ReceiveTick`
  (params (DeltaSeconds :type "Float (single-precision)"))
  (`|ExecutionSequence`
    (:`then_0`
      (if (not (`KismetSystemLibrary.IsValid` (`self.Pawn`)))
        (bind _asbp_pipes_game_mode (cast `/Game/Blueprints/BP_PipesGameMode` (`GameplayStatics.GetGameMode`)))
        (bind _pawn (`/Game/Blueprints/BP_PipesGameMode.GetPawn` _asbp_pipes_game_mode))
        (if (`KismetSystemLibrary.IsValid` _pawn)
          (set `self.Pawn` _pawn))))
    (:`then_1`
      (`self.UpdateCursorPosition`)
      (`self.UpdateCursorEffects`))))

(fn `Choose Candidate Over Next`
  (params (Candidate :type "/Game/Blueprints/Buttons/STRUCT_FocusTarget Structure") (ConsiderObserver :type Boolean))
  (returns (Choose :type Boolean))
  (locals (CandidateInternal :type Boolean) (NextInternal :type Boolean))
  (if (`.Valid_20_591A6B194CD54A976F20ACBAAE539A21` (break `/Game/Blueprints/Buttons/STRUCT_FocusTarget` (`self.NextTarget`)))
    (bind _output_get (set `local.NextInternal` (`|EnumEquality` (`.Type_9_A5EEDFB948529174764A22A5AFD53DBF` (break `/Game/Blueprints/Buttons/STRUCT_FocusTarget` (`self.NextTarget`))) "NewEnumerator1")))
    (bind _output_get_2 (set `local.CandidateInternal` (`|EnumEquality` (`.Type_9_A5EEDFB948529174764A22A5AFD53DBF` (break `/Game/Blueprints/Buttons/STRUCT_FocusTarget` (`local.Candidate`))) "NewEnumerator1")))
    (if (== _output_get_2 _output_get)
      ;[1 1 1] If both options are within their objects, take the one closest to the observer (unless observer is ignored)
      (if (and (`local.NextInternal`) (`local.ConsiderObserver`))
        (if (`KismetSystemLibrary.IsValid` (`self.Pawn`))
          (bind _origin (`/Game/Blueprints/BP_MRPawn.DetectGazeState` (`self.Pawn`)))
          (return (> (`KismetMathLibrary.Vector_DistanceSquared` (`.Point_13_C8C6FDFD4DE0BE172365BD8516CF41AC` (break `/Game/Blueprints/Buttons/STRUCT_FocusTarget` (`self.NextTarget`))) _origin) (`KismetMathLibrary.Vector_DistanceSquared` (`.Point_13_C8C6FDFD4DE0BE172365BD8516CF41AC` (break `/Game/Blueprints/Buttons/STRUCT_FocusTarget` (`local.Candidate`))) _origin)))
          (else
            _)))
      ;[1 1 1] Take the one that's closest to its finger
      (return (> (`.DistanceSq_17_5FBE92264A7E6D39CF347DB86058B320` (break `/Game/Blueprints/Buttons/STRUCT_FocusTarget` (`self.NextTarget`))) (`.DistanceSq_17_5FBE92264A7E6D39CF347DB86058B320` (break `/Game/Blueprints/Buttons/STRUCT_FocusTarget` (`local.Candidate`)))))
      (else
        ;[1 1 1] Only one option is within its object, take that one
        (return (`local.CandidateInternal`))))
    (else
      (return true))))

(fn `Clear Stale Focus`
  (params (Announce :type Boolean))
  (bind _currenttarget_valid (break `/Game/Blueprints/Buttons/STRUCT_FocusTarget` (`self.CurrentTarget`)))
  (bind _nexttarget_valid (break `/Game/Blueprints/Buttons/STRUCT_FocusTarget` (`self.NextTarget`)))
  (bind (_currenttarget_valid_2 _currenttarget_target) (break `/Game/Blueprints/Buttons/STRUCT_FocusTarget` (`self.CurrentTarget`)))
  (bind (_nexttarget_valid_2 _nexttarget_target) (break `/Game/Blueprints/Buttons/STRUCT_FocusTarget` (`self.NextTarget`)))
  (bind _returnvalue (`KismetSystemLibrary.Conv_InterfaceToObject` _currenttarget_target))
  (if _currenttarget_valid
    (if _nexttarget_valid
      (if (!= _returnvalue (`KismetSystemLibrary.Conv_InterfaceToObject` _nexttarget_target))
        (if (and (`KismetSystemLibrary.IsValid` _returnvalue) (`local.Announce`)) :!label _label
          (`/Game/Blueprints/Buttons/Interface_Interactable.UpdateFocusPoint` _currenttarget_target "NewEnumerator1" (0.0 0.0 0.0)))
        (set `self.CurrentTarget` (make `/Game/Blueprints/Buttons/STRUCT_FocusTarget` false)))
      (else
        (goto _label)))))

(fn `ClearFocus`
  (params (Announce :type Boolean))
  (locals (OldTarget :type "/Game/Blueprints/Buttons/Interface_Interactable Interface"))
  (bind (_currenttarget_valid _currenttarget_target) (break `/Game/Blueprints/Buttons/STRUCT_FocusTarget` (`self.CurrentTarget`)))
  (if _currenttarget_valid
    (set `local.OldTarget` _currenttarget_target)
    (set `self.CurrentTarget` (make `/Game/Blueprints/Buttons/STRUCT_FocusTarget` false))
    (set `self.NextTarget` (make `/Game/Blueprints/Buttons/STRUCT_FocusTarget` false))
    (if (`local.Announce`)
      (`/Game/Blueprints/Buttons/Interface_Interactable.UpdateFocusPoint` (`local.OldTarget`) "NewEnumerator2" (0.0 0.0 0.0)))))

(fn `CommitNewFocus`
  (params (Announce :type Boolean))
  (bind (_currenttarget_valid _currenttarget_target _currenttarget_type _currenttarget_cursor) (break `/Game/Blueprints/Buttons/STRUCT_FocusTarget` (`self.CurrentTarget`)))
  (bind (_nexttarget_valid _nexttarget_target _nexttarget_type _nexttarget_cursor _nexttarget_point _nexttarget_normal _nexttarget_distancesq) (break `/Game/Blueprints/Buttons/STRUCT_FocusTarget` (`self.NextTarget`)))
  (bind _nexttarget_valid_2 (break `/Game/Blueprints/Buttons/STRUCT_FocusTarget` (`self.NextTarget`)))
  (if _nexttarget_valid_2
    (set `self.DistToCurrent` (`KismetMathLibrary.Sqrt` _nexttarget_distancesq))
    (if (`local.Announce`)
      (`/Game/Blueprints/Buttons/Interface_Interactable.UpdateFocusPoint` _nexttarget_target "NewEnumerator0" (`self.PointerLocation`))))
  (set `self.CurrentTarget` (`self.NextTarget`))
  (set `self.NextTarget` (make `/Game/Blueprints/Buttons/STRUCT_FocusTarget` false))
  (`self.SetCursorType` (select `bool` _currenttarget_valid :`false` "NewEnumerator0" :`true` _currenttarget_cursor)))

(fn `ConsiderForFocus`
  (params (Candidate :type "/Game/Blueprints/Buttons/Interface_Interactable Interface"))
  (locals (CandidateTarget :type "/Game/Blueprints/Buttons/STRUCT_FocusTarget Structure"))
  (bind _pointerlocation (`self.PointerLocation`))
  (bind (_valid _target _type _cursor _point _normal _distancesq) (break `/Game/Blueprints/Buttons/STRUCT_FocusTarget` (`local.CandidateTarget`)))
  (bind (_type_2 _cursor_2 _point_2 _normal_2) (`/Game/Blueprints/Buttons/Interface_Interactable.QueryFocusPoint` Candidate _pointerlocation))
  (if (`|EnumInequality` _type_2 "NewEnumerator0")
    (bind _output_get (set `local.CandidateTarget` (make `/Game/Blueprints/Buttons/STRUCT_FocusTarget` true (`local.Candidate`) _type_2 _cursor_2 _point_2 _normal_2 (`KismetMathLibrary.Vector_DistanceSquared` _point_2 _pointerlocation))))
    (bind _choose (`self.Choose Candidate Over Next` _output_get true))
    (if _choose
      (if (and (<= (`KismetMathLibrary.DegAcos` (`KismetMathLibrary.Dot_VectorVector` (`self.PointerDefaultNormal`) _normal)) (`self.MaxFocusAngle`)) (<= _distancesq (`KismetMathLibrary.Square` (`self.MaxFocusDistance`))))
        (set `self.NextTarget` (`local.CandidateTarget`))))))

(fn `SetCursorType`
  (params (Type :type "/Game/Blueprints/Buttons/ENUM_CursorType Enum" :default "NewEnumerator0"))
  (bind _arrowmaterial (`self.ArrowMaterial`))
  (if (`|EnumInequality` Type (`self.CursorType`))
    (bind _output_get (set `self.CursorType` (`local.Type`)))
    (switch `/Game/Blueprints/Buttons/ENUM_CursorType` _output_get
      (:`NewEnumerator0`
        (`SceneComponent.SetVisibility` (`self.ArrowPlane`) false false))
      (:`NewEnumerator1`
        (`MaterialInstanceDynamic.SetScalarParameterValue` _arrowmaterial "Solid" -1.0))
      (:`NewEnumerator2`
        (`MaterialInstanceDynamic.SetScalarParameterValue` _arrowmaterial "Solid" 1.0)))))

(fn `UpdateCursorEffects`
  (locals (AltTarget :type "Vector Structure") (NewBehind :type Boolean))
  (bind _currenttarget_valid (break `/Game/Blueprints/Buttons/STRUCT_FocusTarget` (`self.CurrentTarget`)))
  (bind (_currenttarget_valid_2 _currenttarget_target _currenttarget_type _currenttarget_cursor _currenttarget_point _currenttarget_normal) (break `/Game/Blueprints/Buttons/STRUCT_FocusTarget` (`self.CurrentTarget`)))
  (bind (_currenttarget_valid_3 _currenttarget_target_2 _currenttarget_type_2) (break `/Game/Blueprints/Buttons/STRUCT_FocusTarget` (`self.CurrentTarget`)))
  (bind (_currenttarget_valid_4 _currenttarget_target_3 _currenttarget_type_3 _currenttarget_cursor_2 _currenttarget_point_2 _currenttarget_normal_2) (break `/Game/Blueprints/Buttons/STRUCT_FocusTarget` (`self.CurrentTarget`)))
  (bind (_currenttarget_valid_5 _currenttarget_target_4 _currenttarget_type_4 _currenttarget_cursor_3 _currenttarget_point_3) (break `/Game/Blueprints/Buttons/STRUCT_FocusTarget` (`self.CurrentTarget`)))
  (bind _returnvalue (`KismetMathLibrary.FClamp` (/ (`self.DistToCurrent`) (`self.MaxFocusDistance`))))
  (if _currenttarget_valid
    (if (`KismetSystemLibrary.IsValid` (`self.Pawn`))
      (`SceneComponent.SetVisibility` (`self.RingPlane`) true false)
      (`SceneComponent.SetVisibility` (`self.ArrowPlane`) (`|EnumInequality` (`self.CursorType`) "NewEnumerator0") false)
      (set `local.AltTarget` (+ _currenttarget_point_3 (* (`self.PointerDefaultNormal`) 1.25)))
      (bind _origin (`/Game/Blueprints/BP_MRPawn.DetectGazeState` (`self.Pawn`)))
      (if (or (`|EnumInequality` _currenttarget_type_2 "NewEnumerator1") (> (`KismetMathLibrary.Vector_DistanceSquared` _origin (`local.AltTarget`)) (`KismetMathLibrary.Vector_DistanceSquared` _origin (`self.PointerRenderLocation`))))
        (`MaterialInstanceDynamic.SetScalarParameterValue` (`self.RingMaterial`) "OuterRadius" (`KismetMathLibrary.Lerp` (- (`self.Thickness`) (`self.BorderThickness`)) (`self.MaxRadius`) _returnvalue))
        (`self.K2_SetActorLocation` (`self.PointerRenderLocation`))
        (`self.K2_SetActorRotation` (`KismetMathLibrary.RLerp` (`KismetMathLibrary.MakeRotFromXZ` _currenttarget_normal_2 (`KismetMathLibrary.Vector_Up`)) (`KismetMathLibrary.MakeRotFromXZ` (`self.PointerDefaultNormal`) (`KismetMathLibrary.Vector_Up`)) _returnvalue true))
        (else
          (`MaterialInstanceDynamic.SetScalarParameterValue` (`self.RingMaterial`) "OuterRadius" (- (`self.Thickness`) (`self.BorderThickness`)))
          (`self.K2_SetActorLocation` (`local.AltTarget`))
          (`self.K2_SetActorRotation` (`KismetMathLibrary.MakeRotFromXZ` _currenttarget_normal (`KismetMathLibrary.Vector_Up`)))))
      (else
        (`SceneComponent.SetVisibility` (`self.RingPlane`) false false :!label _label)
        (`SceneComponent.SetVisibility` (`self.ArrowPlane`) false false)))
    (else
      (goto _label))))

(fn `UpdateCursorPosition`
  (locals (PrimaryJointRadius :type "Float (double-precision)" :default 0.0) (PrimaryJointLocation :type "Vector Structure" :default (0.0 0.0 0.0)))
  (bind _primaryjointlocation (`local.PrimaryJointLocation`))
  (bind _returnvalue (`KismetMathLibrary.Conv_ByteToInt` (`self.PrimaryJoint`)))
  (bind _motioncontrollerdata (`HeadMountedDisplayFunctionLibrary.GetMotionControllerData` null (`self.Hand`)))
  (bind (_bvalid _devicename _applicationinstanceid _devicevisualtype _handindex _trackingstatus _gripposition _griprotation _aimposition _aimrotation _handkeypositions _handkeyrotations _handkeyradii) (break `XRMotionControllerData` _motioncontrollerdata))
  (bind _returnvalue_2 (and _bvalid (`|EnumEquality` _devicevisualtype "Hand")))
  (bind _output_get (set `self.PointerLocationValid` _returnvalue_2))
  (`SceneComponent.SetVisibility` (`self.Fingertip`) _output_get true)
  (if _returnvalue_2
    (set `local.PrimaryJointRadius` (`|GetArrayItem` _handkeyradii _returnvalue))
    (set `local.PrimaryJointLocation` (`|GetArrayItem` _handkeypositions _returnvalue))
    (bind _returnvalue_3 (`KismetMathLibrary.Normal` (- _primaryjointlocation (`|GetArrayItem` _handkeypositions (`KismetMathLibrary.Conv_ByteToInt` (`self.SecondaryJoint`))))))
    (set `self.PointerDefaultNormal` (* _returnvalue_3 -1))
    (set `self.PointerRenderLocation` (+ _primaryjointlocation (* _returnvalue_3 (* (`local.PrimaryJointRadius`) (`self.RenderRadiusMultiplier`)))))
    (set `self.PointerLocation` (+ (`local.PrimaryJointLocation`) (* _returnvalue_3 (* (`local.PrimaryJointRadius`) (`self.InteractionRadiusMultiplier`)))))))

(fn `UserConstructionScript`)