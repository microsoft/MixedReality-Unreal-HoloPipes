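; Toolbox actor for the pipes game that shows remaining straight, corner and junction pipe counts, plus level and score.
; Labels are dynamic text textures fed into masked material instances, with counts refreshed on contents changes and hidden at zero.
; Tick smoothly yaws the counts toward the pawn's camera.
; Focus changes scale the handle, and carrying spawns a cursor that follows the drop target, with grab and release sounds.
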(event `self.ReceiveBeginPlay`
  (`self.InitializeTextPlanes`))

(event `self.ReceiveTick`
  (params (DeltaSeconds :type "Float (single-precision)"))
  (bind _countsroot (`self.CountsRoot`))
  (bind _returnvalue (`KismetMathLibrary.MakeRotFromZX` (`KismetMathLibrary.Vector_Up`) (- (`SceneComponent.K2_GetComponentLocation` (`/Game/Blueprints/BP_MRPawn.Camera` (`self.Pawn`))) (`SceneComponent.K2_GetComponentLocation` (`self.CountsRoot`)))))
  (if (`KismetSystemLibrary.IsValid` (`self.Pawn`))
    (`SceneComponent.K2_SetWorldRotation` _countsroot (`KismetMathLibrary.RLerp` (`SceneComponent.K2_GetComponentRotation` _countsroot) _returnvalue 0.05 true) false false)
    (else
      (bind _asbp_pipes_game_mode (cast `/Game/Blueprints/BP_PipesGameMode` (`GameplayStatics.GetGameMode`)))
      (bind _pawn (`/Game/Blueprints/BP_PipesGameMode.GetPawn` _asbp_pipes_game_mode))
      (bind _output_get (set `self.Pawn` _pawn))
      (if (`KismetSystemLibrary.IsValid` _output_get)
        (`SceneComponent.K2_SetWorldRotation` (`self.CountsRoot`) _returnvalue false false)))))

(event `self.OnToolboxInitializationComplete`
  (`self.RefreshCounts`))

(event `self.OnToolboxContentsChanged`
  (`self.RefreshCounts`))

(event `self.OnToolboxFocusChanged`
  (bind _returnvalue (`KismetMathLibrary.MakeVector` 0.9 0.9 0.9))
  (bind _focus (`self.Focus`))
  (bind _returnvalue_2 (`SceneComponent.K2_GetComponentLocation` (`self.DefaultSceneRoot`)))
  (bind _returnvalue_3 (`KismetSystemLibrary.IsValid` (`self.DragCursor`)))
  (`SceneComponent.SetRelativeScale3D` (`self.Handle`) (select `EToolboxFocus` _focus :`None` (0.8 0.8 0.8) :`Focused` _returnvalue :`Carried` _returnvalue))
  (if (`|EnumEquality` _focus "Carried")
    (if (not _returnvalue_3)
      (bind _returnvalue_4 (`|SpawnActorFromClass` "/Game/Blueprints/Toolbox/BP_Toolbox_Cursor.BP_Toolbox_Cursor_C" (`self.GetTransform`) "AlwaysSpawn" "OverrideRootScale" null null))
      (set `self.DragCursor` _returnvalue_4)
      (`GameplayStatics.PlaySoundAtLocation` "/Game/Sounds/HoloPipe_Grab.HoloPipe_Grab" _returnvalue_2 (struct) 0.5 1.0 0.0 null null null))
    (elif _returnvalue_3
      (`self.K2_DestroyActor` (`self.DragCursor`))
      (set `self.DragCursor` null)
      (`GameplayStatics.PlaySoundAtLocation` "/Game/Sounds/HoloPipe_Release.HoloPipe_Release" _returnvalue_2 (struct) 2.0 1.0 0.0 null null null))))

(event `self.OnDropTargetChanged`
  (bind _dragcursor (`self.DragCursor`))
  (if (`KismetSystemLibrary.IsValid` _dragcursor)
    (`self.K2_SetActorLocation` _dragcursor (`self.DropTarget`) false false)))

(fn `InitializeTextPlane`
  (params (Width :type Integer) (Height :type Integer) (Mesh :type "StaticMeshComponent Object Reference") (DynamicText :type "/Game/Blueprints/DynamicText/BP_DynamicTextWithMask Object Reference"))
  (`/Game/Blueprints/DynamicText/BP_DynamicTextWithMask.SetTextureSize` DynamicText Width Height false)
  (`/Game/Blueprints/DynamicText/BP_DynamicTextWithMask.SetTextureText` DynamicText "0")
  (bind _returnvalue (`PrimitiveComponent.CreateDynamicMaterialInstance` (`local.Mesh`) 0 "/Game/Materials/MAT_TextWithMask.MAT_TextWithMask" "None"))
  (`MaterialInstanceDynamic.SetTextureParameterValue` _returnvalue "Text" (`/Game/Blueprints/DynamicText/BP_DynamicTextWithMask.Texture` DynamicText))
  (`MaterialInstanceDynamic.SetTextureParameterValue` _returnvalue "Mask" (`/Game/Blueprints/DynamicText/BP_DynamicTextWithMask.Mask` DynamicText)))

(fn `InitializeTextPlanes`
  (`self.InitializeTextPlane` 132 44 (`self.StraightCount`) (`self.StraightCountText`))
  (`self.InitializeTextPlane` 132 44 (`self.CornerCount`) (`self.CornerCountText`))
  (`self.InitializeTextPlane` 132 44 (`self.JunctionCount`) (`self.JunctionCountText`))
  (`self.InitializeTextPlane` 650 44 (`self.Level`) (`self.LevelText`))
  (`self.InitializeTextPlane` 650 44 (`self.Score`) (`self.ScoreText`)))

(fn `RefreshCounts`
  (bind (_straightpipes _cornerpipes _junctionpipes) (break `ToolboxContents` (`self.Contents`)))
  (`SceneComponent.SetVisibility` (`self.StraightCount`) (!= _straightpipes 0) false)
  (`/Game/Blueprints/DynamicText/BP_DynamicTextWithMask.SetTextureText` (`self.StraightCountText`) (`KismetTextLibrary.Conv_IntToText` _straightpipes false false))
  (`SceneComponent.SetVisibility` (`self.CornerCount`) (!= _cornerpipes 0) false)
  (`/Game/Blueprints/DynamicText/BP_DynamicTextWithMask.SetTextureText` (`self.CornerCountText`) (`KismetTextLibrary.Conv_IntToText` _cornerpipes false false))
  (`SceneComponent.SetVisibility` (`self.JunctionCount`) (!= _junctionpipes 0) false)
  (`/Game/Blueprints/DynamicText/BP_DynamicTextWithMask.SetTextureText` (`self.JunctionCountText`) (`KismetTextLibrary.Conv_IntToText` _junctionpipes false false)))

(fn `SetLevel`
  (params (Number :type Integer))
  (`self.SetActorHiddenInGame` false)
  (`/Game/Blueprints/DynamicText/BP_DynamicTextWithMask.SetTextureText` (`self.LevelText`) (`|FormatText` "Level {Number}" Number)))

(fn `SetScore`
  (params (Score :type Integer))
  (bind _returnvalue (!= Score 0))
  (`SceneComponent.SetVisibility` (`self.Score`) _returnvalue false)
  (if _returnvalue
    (`/Game/Blueprints/DynamicText/BP_DynamicTextWithMask.SetTextureText` (`self.ScoreText`) (`KismetTextLibrary.Conv_IntToText` Score))))

(fn `UserConstructionScript`)