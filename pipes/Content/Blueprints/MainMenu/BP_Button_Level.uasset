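; BP_Button_Level is a main menu level button actor that shows a level number and either a star rating or a locked state.
; ChildInitializeFace creates a dynamic material instance on the button face.
; SetLevelDetails stores the level, stars and lock, enables the button when unlocked, and picks the matching face texture.
; It renders the level number into a texture through DynamicText and feeds that to the material's Text parameter.
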(fn `ChildInitializeFace`
  (bind _returnvalue (`PrimitiveComponent.CreateDynamicMaterialInstance` (`self.ButtonFace`) 0 "/Game/Materials/MAT_LevelButton.MAT_LevelButton" "None"))
  (set `self.ButtonFaceMaterial` _returnvalue))

(fn `GetLevelDetails`
  (returns (Level :type Integer) (Stars :type Integer) (Locked :type Boolean))
  (return (`self.Level`) (`self.Stars`) (`self.Locked`)))

(fn `SetLevelDetails`
  (params (NewLevel :type Integer) (NewStars :type Integer) (NewLocked :type Boolean))
  (bind _dynamictext (`self.DynamicText`))
  (set `self.Level` NewLevel)
  (set `self.Stars` NewStars)
  (bind _output_get (set `self.Locked` NewLocked))
  (set `self.Enabled` (not _output_get))
  (`MaterialInstanceDynamic.SetTextureParameterValue` (`self.ButtonFaceMaterial`) "Face" (select `bool` _output_get :`false` (select `int` NewStars :`0` "/Game/Materials/Textures/LevelStars0.LevelStars0" :`1` "/Game/Materials/Textures/LevelStars1.LevelStars1" :`2` "/Game/Materials/Textures/LevelStars2.LevelStars2" :`3` "/Game/Materials/Textures/LevelStars3.LevelStars3" :`4` "/Game/Materials/Textures/LevelStars4.LevelStars4" :!type "Texture Object Reference") :`true` "/Game/Materials/Textures/Locked.Locked"))
  (`/Game/Blueprints/DynamicText/BP_DynamicText.SetTextureSize` _dynamictext 88 44 false)
  (`/Game/Blueprints/DynamicText/BP_DynamicText.SetTextureText` _dynamictext (`KismetTextLibrary.Conv_IntToText` (`local.NewLevel`) false false))
  (`MaterialInstanceDynamic.SetTextureParameterValue` (`self.ButtonFaceMaterial`) "Text" (`/Game/Blueprints/DynamicText/BP_DynamicText.Texture` _dynamictext)))

(fn `UserConstructionScript`
  (`parent.UserConstructionScript`))